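; BP_Obstacle is an obstacle Blueprint whose Cube component can be temporarily removed by holding the C key.
; Pressing C hides the cube and disables its collision and component tick, while releasing restores visibility, query-and-physics collision and ticking.
; Each transition prints a debug string, though the labels read inverted: "Cube" when hidden, "Gone" when restored.
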(event EventBeginPlay)

(event Collision|EventActorBeginOverlap
  (params (OtherActor :type Actor%20Object%20Reference)))

(event EventTick
  (params (DeltaSeconds :type Float%20%28single-precision%29)))

(event Input|KeyboardEvents|C
  (params (Key :type Key%20Structure :default "None"))
  (bind _cube (Variables|Default|GetCube))
  (bind _cube_2 (Variables|Default|GetCube))
  (:Pressed
    (Rendering|SetVisibility (Variables|Default|GetCube) false false)
    (Collision|SetCollisionEnabled _cube "NoCollision")
    (Components|Tick|SetComponentTickEnabled _cube false)
    (Development|PrintString "Cube"))
  (:Released
    (Rendering|SetVisibility (Variables|Default|GetCube) true false)
    (Collision|SetCollisionEnabled _cube_2 "QueryAndPhysics")
    (Components|Tick|SetComponentTickEnabled _cube_2 true)
    (Development|PrintString "Gone")))

(fn ConstructionScript)