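; Monkey pirate NPC that runs a sword-insertion quest through the dialogue state index of its parent class.
; Before dialogue starts, it inserts the final sword if flagged, otherwise one collected sword per conversation, counting toward the total needed.
; Each insertion picks a dialogue state for progress, all swords inserted or final sword.
; Post-update logic advances these states once the castle quest is complete.
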(event Custom|Add%20Sword
  ;[1 1 1] Add Sword
  (Math|Integer|IncrementInt (Variables|Default|GettotalCollected)))

(event Custom|Insert%20Sword
  ;[1 1 1] Insert Sword
  (if (not (Variables|Default|GetfinalSword))
    (bind _result (Math|Integer|IncrementInt (Variables|Default|GettotalInserted))
      (:%20%20
        (if (== _result (Variables|Default|GettotalNeeded))
          (Variables|Default|SetstateIndex 4)
          (else
            (Variables|Default|SetstateIndex 3)))))
    (else
      (Variables|Default|SetfinalSword false)
      (Variables|Default|SetstateIndex 6)))
  (CallFunction|StartDialogue))

(event EventPostStatesUpdate
  ;[1 1 1] Quest Update Changes
  (if (Variables|Default|GetcastleQuestComplete)
    (if (== (Variables|Default|GetstateIndex) 1)
      (Variables|Default|SetstateIndex 2)
      (elif (and (== (Variables|Default|GetstateIndex) 3) (== (Variables|Default|GettotalCollected) 0))
        (Variables|Default|SetstateIndex 2)
        (elif (== (Variables|Default|GetstateIndex) 4)
          (Variables|Default|SetstateIndex 5)
          (elif (== (Variables|Default|GetstateIndex) 6)
            (Variables|Default|SetstateIndex 7)))))))

(event EventPreStartDialogue
  (bind _totalcollected (Variables|Default|GettotalCollected))
  ;[1 1 1] Insert Sword Check
  (if (Variables|Default|GetfinalSword)
    (CallFunction|InsertSword :!label _label)
    (elif (> _totalcollected 0)
      (Math|Integer|DecrementInt _totalcollected
        (:%20%20
          (goto _label)))
      (else
        (CallFunction|StartDialogue)))))

(fn ConstructionScript
  (|CallParentFunction))