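; Dialogue NPC Blueprint that serves as a quest trigger, marking its quest completed when the QuestTrigger event fires.
; After a states update, it moves CurrentState from the initial first-encounter state to the next one and sets DialogueIndex from the DialogueStates entry for the current state.
; QuestReward is left empty, and the construction script only runs the parent's.
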(event Custom|Quest%20Trigger
  ;[1 1 1] Quest Trigger
  (Variables|Default|SetquestCompleted true))

(event Custom|Quest%20Reward)

(event EventPostStatesUpdate
  ;[1 1 1] First Encounter State Change
  (if (== (Variables|Default|GetcurrentState) 0)
    (Variables|Default|SetcurrentState 1))
  (Variables|Default|SetdialogueIndex (Utilities|Array|Get(acopy) (Variables|Default|GetDialogue%20States) (Variables|Default|GetcurrentState))))

(fn ConstructionScript
  (|CallParentFunction))