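; Guard NPC dialogue blueprint that hands out and advances the princess quest.
; After each state update, the first state flags the princess collection-quest NPC as accepted and moves its dialogue forward.
; That step also resizes the guard's collision sphere and moves its player teleport point.
; A later state advances once more, and the dialogue index always follows the current state.
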(event EventPostStatesUpdate
  ;[1 1 1] Start Princess Quest
  (if (== (Variables|Default|GetcurrentState) 0)
    (Variables|Default|SetcurrentState 1)
    (bind _returnvalue (Actor|GetActorOfClass "/Game/Dialogue_Quests/BP_NPC_CollectionQuest_Princess.BP_NPC_CollectionQuest_Princess_C"))
    (Variables|/Game/Dialogue_Quests/BP_NPC_CollectionQuest_Princess.BP_NPC_CollectionQuest_Princess_C|SetquestAccepted _returnvalue true)
    (Variables|/Game/Dialogue_Quests/BP_NPC.BP_NPC_C|SetcurrentState _returnvalue 2)
    (Variables|/Game/Dialogue_Quests/BP_NPC.BP_NPC_C|SetdialogueIndex _returnvalue (Utilities|Array|Get(acopy) (Variables|/Game/Dialogue_Quests/BP_NPC.BP_NPC_C|GetDialogue%20States _returnvalue) (Variables|/Game/Dialogue_Quests/BP_NPC.BP_NPC_C|GetcurrentState _returnvalue)))
    (Components|Sphere|SetSphereRadius (Variables|Default|GetSphereCollision) 175.0 true)
    (Transformation|SetRelativeLocation (Variables|Default|GetPlayerTeleport) "0,160.000000, 0" false false)
    (elif (== (Variables|Default|GetcurrentState) 2)
      (Variables|Default|SetcurrentState 3)))
  (Variables|Default|SetdialogueIndex (Utilities|Array|Get(acopy) (Variables|Default|GetDialogue%20States) (Variables|Default|GetcurrentState))))

(fn ConstructionScript
  (|CallParentFunction))