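; BP_NPC_CollectionQuest is a quest NPC Blueprint whose dialogue follows collection progress through a numbered state.
; PostStatesUpdate advances the state from 0 to 1 after the first encounter.
; QuestUpdate increments TotalCollected and sets state 2 on every call, since its branch is always true and the TotalNeeded comparison is unused.
; Both events then set DialogueIndex from the DialogueStates entry for the current state.
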(event Custom|Quest%20Update
  ;[1 1 1] Quest Update
  (Math|Integer|IncrementInt (Variables|Default|GettotalCollected)
    (:%20%20
      (if true
        (Variables|Default|SetcurrentState 2))
      (Variables|Default|SetdialogueIndex (Utilities|Array|Get(acopy) (Variables|Default|GetDialogue%20States) (Variables|Default|GetcurrentState))))))

(event EventPostStatesUpdate
  ;[1 1 1] First Encounter Update
  (if (== (Variables|Default|GetcurrentState) 0)
    (Variables|Default|SetcurrentState 1))
  (Variables|Default|SetdialogueIndex (Utilities|Array|Get(acopy) (Variables|Default|GetDialogue%20States) (Variables|Default|GetcurrentState))))

(fn ConstructionScript
  (|CallParentFunction))