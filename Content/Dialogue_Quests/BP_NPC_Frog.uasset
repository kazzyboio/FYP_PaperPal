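; Frog NPC for the princess quest, offering dialogue only while BP_NPC_Princess has StateIndex 3.
; Collision toggles a text prompt or auto-starts dialogue, and activation hides the prompt and calls PlayerAdjustments.
; Ending dialogue blends the camera back to the player, plays a timeline, resets dialogue state and advances the princess quest.
; During a screen fade, it spawns a Static_Frog at a target point, restores movement input and destroys itself.
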(event EventEndDialogue
  ;[1 1 1] End Dialogue
  (Widget|RemovefromParent (Variables|Default|GetdialogueUI))
  (Game|Player|SetViewTargetwithBlend (Game|GetPlayerController 0) (Game|GetPlayerCharacter 0) (Variables|Default|GetblendTime) "VTBlend_Linear" 0.0 false)
  (Timeline|Timeline_2 PlayFromStart
    (:Finished
      (Variables|Default|SetspeakerIndex 0)
      (Variables|Default|SetdialogueStart false)
      (CallFunction|PostStatesUpdate))))

(event EventPostStatesUpdate
  ;[1 1 1] Update Princess Quest
  (bind _returnvalue (Actor|GetActorOfClass "/Game/Dialogue_Quests/BP_NPC_Princess.BP_NPC_Princess_C"))
  (Default|QuestUpdate _returnvalue)
  (CallFunction|StartFade)
  (Utilities|FlowControl|Delay 1.0)
  (Rendering|SetActorHiddenInGame true)
  (bind _returnvalue_2 (Game|SpawnActorfromClass "/Game/Dialogue_Quests/Static_Frog.Static_Frog_C" (Variables|Default|GetSpawn%20Transform) "Undefined" 0 0))
  (Transformation|SetActorRelativeLocation _returnvalue_2 (Transformation|GetWorldLocation (Variables|/Script/Engine.Actor|GetRootComponent (Variables|Default|GettargetPoint))))
  (Utilities|FlowControl|Delay 1.0)
  (CallFunction|EndFade)
  (Input|SetIgnoreMoveInput (Game|GetPlayerController 0) false)
  (Actor|DestroyActor))

(event EventActivateDialogue
  ;[1 1 1] Check Quest Accepted
  (bind _returnvalue (Actor|GetActorOfClass "/Game/Dialogue_Quests/BP_NPC_Princess.BP_NPC_Princess_C"))
  (if (== (Variables|/Game/Dialogue_Quests/BP_NPC.BP_NPC_C|GetstateIndex _returnvalue) 3)
    (Development|SetHiddeninGame (Variables|Default|GetTextRender) true false)
    (CallFunction|PlayerAdjustments)))

(event EventEnterCollision
  ;[1 1 1] Check Quest Accepted
  (bind _returnvalue (Actor|GetActorOfClass "/Game/Dialogue_Quests/BP_NPC_Princess.BP_NPC_Princess_C"))
  (if (== (Variables|/Game/Dialogue_Quests/BP_NPC.BP_NPC_C|GetstateIndex _returnvalue) 3)
    (if (Variables|Default|GetautoActivate)
      (Utilities|FlowControl|Delay 0.1)
      (Variables|Default|SetautoActivate false)
      (Development|SetHiddeninGame (Variables|Default|GetTextRender) true false)
      (CallFunction|PlayerAdjustments)
      (else
        (Development|SetHiddeninGame (Variables|Default|GetTextRender) false false)))))

(event EventExitCollision
  ;[1 1 1] Check Quest Accepted
  (bind _returnvalue (Actor|GetActorOfClass "/Game/Dialogue_Quests/BP_NPC_Princess.BP_NPC_Princess_C"))
  (if (== (Variables|/Game/Dialogue_Quests/BP_NPC.BP_NPC_C|GetstateIndex _returnvalue) 3)
    (Development|SetHiddeninGame (Variables|Default|GetTextRender) true false)))

(fn ConstructionScript
  (|CallParentFunction))