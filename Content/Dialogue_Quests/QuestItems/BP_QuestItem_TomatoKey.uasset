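; Tomato key quest item that, when picked up, flags the key as obtained on Mr. Tomato Head, makes the player stinky and shows the key as a back item.
; A one-time update spawns a self-dialogue actor at the player, filled from the NPC script data table, switching its state if the quest is not yet accepted.
; It then plays the collect effect, hides the mesh and popup, and destroys itself after a short delay.
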(event EventBeginPlay
  (Components|Activation|Deactivate (Variables|Default|GetNS_CollectItem)))

(event EventPickUpItem
  ;[1 1 1] Quest Accepeted Check
  (CallFunction|PickUpUpdate)
  (bind _returnvalue (Actor|GetActorOfClass "/Game/PlayerCharacter/BP_Player.BP_Player_C"))
  (Default|SpawnBackItemKey _returnvalue))

(event EventPickUpUpdate
  (bind _returnvalue (Game|GetPlayerCharacter 0))
  (bind _rootcomponent (Variables|/Script/Engine.Actor|GetRootComponent _returnvalue))
  ;[1 1 1] Got Key Update
  (Utilities|FlowControl|DoOnce false
    (:Completed
      (bind _returnvalue_2 (Actor|GetActorOfClass "/Game/Dialogue_Quests/NPCs/BP_NPC_MrTomatoHead.BP_NPC_MrTomatoHead_C"))
      (Variables|/Game/Dialogue_Quests/NPCs/BP_NPC_MrTomatoHead.BP_NPC_MrTomatoHead_C|SetkeyGot _returnvalue_2 true)
      (bind _returnvalue_3 (Actor|GetActorOfClass "/Game/PlayerCharacter/BP_Player.BP_Player_C"))
      (Variables|/Game/PlayerCharacter/BP_Player.BP_Player_C|SetisStinky _returnvalue_3 true)
      (Default|StinkyEffect _returnvalue_3)
      (bind _output_get (Variables|Default|SetSpawn%20Transform (Math|Transform|MakeTransform (Transformation|GetWorldLocation _rootcomponent) (Transformation|GetWorldRotation _rootcomponent) "1.000000,1.000000,1.000000")))
      (bind _returnvalue_4 (Game|SpawnActorfromClass "/Game/Dialogue_Quests/NPCs/BP_NPC_SelfDialogue.BP_NPC_SelfDialogue_C" _output_get "Undefined" 0 0))
      (bind _output_get_2 (Variables|/Game/Dialogue_Quests/NPCs/BP_NPC.BP_NPC_C|SetRow%20Name _returnvalue_4 "Self_Dialogue_Stinky_Pickup"))
      (bind _returnvalue_5 (Utilities|GetDataTableRow "/Game/Dialogue_Quests/DataTables/DT_NPCScripts.DT_NPCScripts" _output_get_2)
        (:then
          (Variables|/Game/Dialogue_Quests/NPCs/BP_NPC.BP_NPC_C|SetDialogue%20States _returnvalue_4 (.dialogueStates (Utilities|Struct|BreakStruct_NPCInfo _returnvalue_5)))
          (Variables|/Game/Dialogue_Quests/NPCs/BP_NPC.BP_NPC_C|SetType%20Speed _returnvalue_4 (.typeSpeed (Utilities|Struct|BreakStruct_NPCInfo _returnvalue_5)))
          (if (not (Variables|/Game/Dialogue_Quests/NPCs/BP_NPC_MrTomatoHead.BP_NPC_MrTomatoHead_C|GetkeyQuestAccepted _returnvalue_2))
            (Variables|/Game/Dialogue_Quests/NPCs/BP_NPC.BP_NPC_C|SetstateIndex _returnvalue_4 1))
          (Components|Activation|Activate (Variables|Default|GetNS_CollectItem) false)
          (Rendering|SetVisibility (Variables|Default|GetStaticMesh) false false)
          (bind _asbp_player (Utilities|Casting|CastToBP_Player (Game|GetPlayerCharacter 0)))
          (Default|HIDEUI (Variables|/Game/PlayerCharacter/BP_Player.BP_Player_C|GetPOP%20up _asbp_player))
          (Utilities|FlowControl|Delay 0.7)
          (Actor|DestroyActor))))))

(fn ConstructionScript
  (|CallParentFunction))