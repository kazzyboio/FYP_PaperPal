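; BP_QuestItem_Collectable is a snack collectable that stays hidden and non-colliding until SpawnSnack reveals it with a glow and spin.
; The first player overlap plays a sound and timeline-driven rise-and-spin, then a collect Niagara effect and an input-device-specific WB_Tutorial notification.
; It then unlocks the WB_Collectables_Button matching its RowName, found by searching all widgets of that class, and destroys itself.
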(event OnComponentBeginOverlap(SphereCollisionRadius)
  (params (OverlappedComponent :type Primitive%20Component%20Object%20Reference) (OtherActor :type Actor%20Object%20Reference) (OtherComp :type Primitive%20Component%20Object%20Reference) (OtherBodyIndex :type Integer) (bFromSweep :type Boolean) (SweepResult :type Hit%20Result%20Structure%20%28by%20ref%29))
  (Utilities|Casting|CastToBP_Player OtherActor)
  (Utilities|FlowControl|DoOnce false
    (:Completed
      (Audio|PlaySound2D (Variables|Default|GetCollectSound) 1.0 1.0 0.0 0 0)
      (Components|Activation|Deactivate (Variables|Default|GetNS_ItemGlow))
      (CallFunction|StopSpinANi)
      (bind _newtrack_0 (Timeline|PickUpAni Play)
        (:Update
          (Transformation|SetRelativeLocation (Variables|Default|GetStaticMesh) (Math|Vector|MakeVector 0.0 0.0 _newtrack_0) false false)
          (bind _rotate (Timeline|PickupSpin Play)
            (:Update
              (Transformation|SetRelativeRotation (Variables|Default|GetStaticMesh) (Math|Rotator|MakeRotator 9e+01 0.0 _rotate) false false)
              (Utilities|FlowControl|Delay 1.4)
              (Rendering|SetVisibility (Variables|Default|GetStaticMesh) false false)
              (Components|Activation|Activate (Variables|Default|GetNS_CollectItem) false)
              (Utilities|FlowControl|Delay 0.7)
              (bind _asbp_player (Utilities|Casting|CastToBP_Player (Game|GetPlayerCharacter 0)))
              (switch Utilities|FlowControl|Switch|SwitchonInputDevice (Variables|/Game/PlayerCharacter/BP_Player.BP_Player_C|GetCurrentInputDevice _asbp_player)
                (:NewEnumerator0
                  (bind _returnvalue (UserInterface|CreateWidget "/Game/Assets/UI/WB/WB_Tutorial.WB_Tutorial_C"))
                  (UserInterface|Viewport|AddtoViewport _returnvalue 0)
                  (Default|CollectableNotiKBM _returnvalue))
                (:NewEnumerator1
                  (bind _returnvalue_2 (UserInterface|CreateWidget "/Game/Assets/UI/WB/WB_Tutorial.WB_Tutorial_C"))
                  (UserInterface|Viewport|AddtoViewport _returnvalue_2 0)
                  (Default|CollectibleNotiPad _returnvalue_2)))
              (CallFunction|PickUpItem))))))))

(event OnComponentEndOverlap(SphereCollisionRadius)
  (params (OverlappedComponent :type Primitive%20Component%20Object%20Reference) (OtherActor :type Actor%20Object%20Reference) (OtherComp :type Primitive%20Component%20Object%20Reference) (OtherBodyIndex :type Integer)))

(event Custom|SpinAnimation
  (bind _rotate (Timeline|RotationAni Play)
    (:Update
      (Transformation|SetRelativeRotation (Variables|Default|GetStaticMesh) (Math|Rotator|MakeRotator 9e+01 0.0 _rotate) false false))))

(event Custom|SpawnSnack
  (Rendering|SetVisibility (Variables|Default|GetStaticMesh) true false)
  (Collision|SetCollisionProfileName (Variables|Default|GetSphereCollisionRadius) "OverlapAll" true :!class /Script/Engine.PrimitiveComponent)
  (CallFunction|SpinAnimation))

(event Custom|StopSpinANi
  (bind _rotate (Timeline|RotationAni Stop)
    (:Update
      (Transformation|SetRelativeRotation (Variables|Default|GetStaticMesh) (Math|Rotator|MakeRotator 9e+01 0.0 _rotate) false false))))

(event EventPickUpUpdate
  ;[1 1 1] Pick Up Collectable, Check and Unlock Corresponding Button
  (bind _foundwidgets (Widget|GetAllWidgetsOfClass "/Game/Assets/UI/WB/WB_Collectables_Button.WB_Collectables_Button_C" false))
  (bind _array_element (Utilities|Array|ForEachLoopwithBreak _foundwidgets :!label _label)
    (:LoopBody
      (if (== (Variables|/Game/Assets/UI/WB/WB_Collectables_Button.WB_Collectables_Button_C|GetrowName _array_element) (Variables|Default|GetrowName))
        (Default|Unlock _array_element)
        (goto _label Break)))))

(event EventBeginPlay
  (Rendering|SetVisibility (Variables|Default|GetStaticMesh) false false)
  (Collision|SetCollisionProfileName (Variables|Default|GetSphereCollisionRadius) "NoCollision" true :!class /Script/Engine.PrimitiveComponent))

(event EventPickUpItem
  (CallFunction|PickUpUpdate)
  (Actor|DestroyActor))

(fn ConstructionScript
  (Rendering|Material|SetMaterial (Variables|Default|GetStaticMesh) 0 (Variables|Default|GetSnackTexture)))