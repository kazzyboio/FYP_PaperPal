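; Collectible sword for the Monkey Pirate quest, which stays inert until the player accepts the quest from BP_NPC_MonkeyPirate.
; Tick polls that NPC to switch on highlight and glow once, and the same check gates parent collision events and pickup.
; Pickup plays effects, hides the sword and popup, increments the NPC's count, then destroys itself.
; Reaching the required total spawns a table-driven self-dialogue actor, noted as broken.
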(event EventPickUpItem
  (bind _staticmesh (Variables|Default|GetStaticMesh))
  ;[1 1 1] Quest Accepeted Check
  (bind _returnvalue (Actor|GetActorOfClass "/Game/Dialogue_Quests/NPCs/BP_NPC_MonkeyPirate.BP_NPC_MonkeyPirate_C"))
  (if (Variables|/Game/Dialogue_Quests/NPCs/BP_NPC_MonkeyPirate.BP_NPC_MonkeyPirate_C|GetquestAccepted _returnvalue)
    (Utilities|FlowControl|DoOnce false
      (:Completed
        (Audio|PlaySound2D "/Game/Assets/SFX/SFX_Pop_2.SFX_Pop_2" 1.0 1.0 0.0 0 0)
        (CallFunction|PickUpUpdate)
        (Components|Activation|Activate (Variables|Default|GetNS_CollectItem) false)
        (Rendering|SetVisibility _staticmesh false false)
        (Collision|SetCollisionProfileName _staticmesh "NoCollision" true :!class /Script/Engine.PrimitiveComponent)
        (bind _asbp_player (Utilities|Casting|CastToBP_Player (Game|GetPlayerCharacter 0)))
        (Default|HIDEUI (Variables|/Game/PlayerCharacter/BP_Player.BP_Player_C|GetPOP%20up _asbp_player))
        (Utilities|FlowControl|Delay 0.7)
        (Actor|DestroyActor)))))

(event EventPickUpUpdate
  (bind _returnvalue (Game|GetPlayerCharacter 0))
  (bind _rootcomponent (Variables|/Script/Engine.Actor|GetRootComponent _returnvalue))
  ;[1 1 1] Sword Number Update
  (bind _returnvalue_2 (Actor|GetActorOfClass "/Game/Dialogue_Quests/NPCs/BP_NPC_MonkeyPirate.BP_NPC_MonkeyPirate_C"))
  (Default|AddSword _returnvalue_2)
  ;[1 1 1] Self Dialogue on 3rd sword (Not implemented/broken)
  (if (== (+ (Variables|/Game/Dialogue_Quests/NPCs/BP_NPC_MonkeyPirate.BP_NPC_MonkeyPirate_C|GettotalCollected _returnvalue_2) (Variables|/Game/Dialogue_Quests/NPCs/BP_NPC_MonkeyPirate.BP_NPC_MonkeyPirate_C|GettotalInserted _returnvalue_2)) (Variables|/Game/Dialogue_Quests/NPCs/BP_NPC_MonkeyPirate.BP_NPC_MonkeyPirate_C|GettotalNeeded _returnvalue_2))
    (bind _output_get (Variables|Default|SetSpawn%20Transform (Math|Transform|MakeTransform (Transformation|GetWorldLocation _rootcomponent) (Transformation|GetWorldRotation _rootcomponent) "1.000000,1.000000,1.000000")))
    (bind _returnvalue_3 (Game|SpawnActorfromClass "/Game/Dialogue_Quests/NPCs/BP_NPC_SelfDialogue.BP_NPC_SelfDialogue_C" _output_get "Undefined" 0 0))
    (bind _output_get_2 (Variables|/Game/Dialogue_Quests/NPCs/BP_NPC.BP_NPC_C|SetRow%20Name _returnvalue_3 "Self_Dialogue_Sword"))
    (bind _returnvalue_4 (Utilities|GetDataTableRow "/Game/Dialogue_Quests/DataTables/DT_NPCScripts.DT_NPCScripts" _output_get_2)
      (:then
        (Variables|/Game/Dialogue_Quests/NPCs/BP_NPC.BP_NPC_C|SetDialogue%20States _returnvalue_3 (.dialogueStates (Utilities|Struct|BreakStruct_NPCInfo _returnvalue_4)))
        (Variables|/Game/Dialogue_Quests/NPCs/BP_NPC.BP_NPC_C|SetType%20Speed _returnvalue_3 (.typeSpeed (Utilities|Struct|BreakStruct_NPCInfo _returnvalue_4)))))))

(event EventEnterCollision
  ;[1 1 1] Collision Events Check
  (bind _returnvalue (Actor|GetActorOfClass "/Game/Dialogue_Quests/NPCs/BP_NPC_MonkeyPirate.BP_NPC_MonkeyPirate_C"))
  (if (Variables|/Game/Dialogue_Quests/NPCs/BP_NPC_MonkeyPirate.BP_NPC_MonkeyPirate_C|GetquestAccepted _returnvalue)
    (|CallParentFunction)))

(event EventExitCollision
  ;[1 1 1] Collision Events Check
  (bind _returnvalue (Actor|GetActorOfClass "/Game/Dialogue_Quests/NPCs/BP_NPC_MonkeyPirate.BP_NPC_MonkeyPirate_C"))
  (if (Variables|/Game/Dialogue_Quests/NPCs/BP_NPC_MonkeyPirate.BP_NPC_MonkeyPirate_C|GetquestAccepted _returnvalue)
    (|CallParentFunction)))

(event EventTick
  (params (DeltaSeconds :type Float%20%28single-precision%29))
  ;[1 1 1] Sword Particles
  (if (not (Variables|Default|GetglowActivate))
    (bind _returnvalue (Actor|GetActorOfClass "/Game/Dialogue_Quests/NPCs/BP_NPC_MonkeyPirate.BP_NPC_MonkeyPirate_C"))
    (if (Variables|/Game/Dialogue_Quests/NPCs/BP_NPC_MonkeyPirate.BP_NPC_MonkeyPirate_C|GetquestAccepted _returnvalue)
      (Rendering|Material|SetScalarParameterValueonMaterials (Variables|Default|GetStaticMesh) "Highlight" 1.0)
      (Components|Activation|Activate (Variables|Default|GetNS_ItemGlow) false)
      (Variables|Default|SetglowActivate true))))

(fn ConstructionScript
  (|CallParentFunction))