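; Hay pickup for the farm pig NPC's quest, which stays inactive until that quest is accepted.
; Tick polls the pig's QuestAccepted flag, then turns on the material highlight and Niagara glow once.
; Collision enter and exit pass to the parent only while the quest is accepted.
; Pickup calls QuestUpdate on the pig and destroys the hay, with every event finding the pig through GetActorOfClass.
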(event EventPickUpItem
  ;[1 1 1] Quest Accepeted Check
  (bind _returnvalue (Actor|GetActorOfClass "/Game/Dialogue_Quests/NPCs/BP_NPC_FarmAnimal_Pig.BP_NPC_FarmAnimal_Pig_C"))
  (if (Variables|/Game/Dialogue_Quests/NPCs/BP_NPC_FarmAnimal_Pig.BP_NPC_FarmAnimal_Pig_C|GetquestAccepted _returnvalue)
    (CallFunction|PickUpUpdate)
    (Actor|DestroyActor)))

(event EventPickUpUpdate
  ;[1 1 1] Hay Number Update
  (bind _returnvalue (Actor|GetActorOfClass "/Game/Dialogue_Quests/NPCs/BP_NPC_FarmAnimal_Pig.BP_NPC_FarmAnimal_Pig_C"))
  (Default|QuestUpdate _returnvalue))

(event EventEnterCollision
  ;[1 1 1] Collision Events Check
  (bind _returnvalue (Actor|GetActorOfClass "/Game/Dialogue_Quests/NPCs/BP_NPC_FarmAnimal_Pig.BP_NPC_FarmAnimal_Pig_C"))
  (if (Variables|/Game/Dialogue_Quests/NPCs/BP_NPC_FarmAnimal_Pig.BP_NPC_FarmAnimal_Pig_C|GetquestAccepted _returnvalue)
    (|CallParentFunction)))

(event EventExitCollision
  ;[1 1 1] Collision Events Check
  (bind _returnvalue (Actor|GetActorOfClass "/Game/Dialogue_Quests/NPCs/BP_NPC_FarmAnimal_Pig.BP_NPC_FarmAnimal_Pig_C"))
  (if (Variables|/Game/Dialogue_Quests/NPCs/BP_NPC_FarmAnimal_Pig.BP_NPC_FarmAnimal_Pig_C|GetquestAccepted _returnvalue)
    (|CallParentFunction)))

(event EventTick
  (params (DeltaSeconds :type Float%20%28single-precision%29))
  ;[1 1 1] Sword Particles
  (if (not (Variables|Default|GetglowActivate))
    (bind _returnvalue (Actor|GetActorOfClass "/Game/Dialogue_Quests/NPCs/BP_NPC_FarmAnimal_Pig.BP_NPC_FarmAnimal_Pig_C"))
    (if (Variables|/Game/Dialogue_Quests/NPCs/BP_NPC_FarmAnimal_Pig.BP_NPC_FarmAnimal_Pig_C|GetquestAccepted _returnvalue)
      (Rendering|Material|SetScalarParameterValueonMaterials (Variables|Default|GetStaticMesh) "Highlight" 1.0)
      (Components|Activation|Activate (Variables|Default|GetNS_ItemGlow) false)
      (Variables|Default|SetglowActivate true))))

(fn ConstructionScript
  (|CallParentFunction))