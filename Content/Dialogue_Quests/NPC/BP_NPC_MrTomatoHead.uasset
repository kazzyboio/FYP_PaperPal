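; Mr. Tomato Head NPC that runs a staged gate encounter and introduces a tutorial, built on a parent dialogue NPC.
; StateIndex advances after the first state update, widening the trigger sphere, then on gate opening, when the NPC turns and starts dialogue.
; The following update fades, teleports the NPC to a target point, restores movement through the parent and shows the animated tutorial widget.
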(event Custom|Gate%20Opened
  ;[1 1 1] Gate Event
  (if (== (Variables|Default|GetstateIndex) 1)
    (Variables|Default|SetstateIndex 2)
    (Utilities|FlowControl|Delay 0.5)
    (Transformation|SetActorRotation "0,195.000000, 0")
    (Variables|Default|SetpastGate true)
    (CallFunction|ActivateDialogue)))

(event EventReactivateMovement
  ;[1 1 1] Reactivate Movement
  (if (not (== (Variables|Default|GetstateIndex) 2))
    (|CallParentFunction)))

(event EventPostStatesUpdate
  ;[1 1 1] First Encounter Updates
  (if (not (== (Variables|Default|GetstateIndex) 2))
    (if (== (Variables|Default|GetstateIndex) 0)
      (Variables|Default|SetstateIndex 1)
      (Components|Sphere|SetSphereRadius (Variables|Default|GetSphereCollision) 2e+02 true))
    (else
      ;[1 1 1] Teleport
      (Variables|Default|SetdialogueStart true)
      (CallFunction|StartFade)
      (Utilities|FlowControl|Delay (Variables|Default|GetfadeDelay))
      (Transformation|SetActorRelativeLocation (Transformation|GetWorldLocation (Variables|/Script/Engine.Actor|GetRootComponent (Variables|Default|GettargetPoint))))
      (Transformation|SetActorRotation "0.000000,295.000000,0.000000")
      (Utilities|FlowControl|Delay (Variables|Default|GetfadeDelay))
      (|CallParentFunction)
      (Variables|Default|SetstateIndex 3)
      (Variables|Default|SetdialogueStart false)
      ;[1 1 1] Tutorial Pop Up
      (bind _returnvalue (UserInterface|CreateWidget "/Game/Assets/PlaceHolderAssets/WB_Tutorial.WB_Tutorial_C"))
      (UserInterface|Viewport|AddtoViewport _returnvalue 0)
      (Default|RollTutorialAnimation _returnvalue))))

(fn ConstructionScript
  (|CallParentFunction))