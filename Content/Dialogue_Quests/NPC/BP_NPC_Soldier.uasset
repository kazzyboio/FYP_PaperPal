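; Soldier quest NPC built on a parent dialogue class, using a state index to track first encounters, quest acceptance and completion of a collection quest.
; QuestUpdate counts collected items and sets the completion state, in which PostStatesUpdate destroys the soldier.
; A dialogue line in that state pauses dialogue, fades, hides the soldier, spawns Static_Princess at a target point, advances the guards' state, then resumes dialogue.
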(event Custom|Quest%20Update
  ;[1 1 1] Quest Update
  (bind _result (Math|Integer|IncrementInt (Variables|Default|GettotalCollected))
    (:%20%20
      (if (== _result (Variables|Default|GettotalNeeded))
        (Variables|Default|SetstateIndex 4)))))

(event EventDialogueEvent
  (bind _dialogueui (Variables|Default|GetdialogueUI))
  ;[1 1 1] Quest Finish Teleport
  (if (and (== 4 (Variables|Default|GetstateIndex)) (== 2 (Variables|Default|GetdialogueIndex)))
    (Variables|Default|SetdialoguePlaying false)
    (Default|DespawnWidget (Variables|Default|GetdialogueUI))
    (CallFunction|StartFade)
    (Utilities|FlowControl|Delay (Variables|Default|GetfadeDelay))
    (Rendering|SetActorHiddenInGame true)
    (bind _returnvalue (Game|SpawnActorfromClass "/Game/Dialogue_Quests/Static_Princess.Static_Princess_C" (Variables|Default|GetSpawn%20Transform) "Undefined" 0 0))
    (Transformation|SetActorRelativeLocation _returnvalue (Transformation|GetWorldLocation (Variables|/Script/Engine.Actor|GetRootComponent (Variables|Default|GettargetPoint))))
    (bind _returnvalue_2 (Actor|GetActorOfClass "/Game/Dialogue_Quests/NPC/BP_NPC_Guards.BP_NPC_Guards_C"))
    (Variables|/Game/Dialogue_Quests/NPC/BP_NPC.BP_NPC_C|SetstateIndex _returnvalue_2 2)
    (Utilities|FlowControl|Delay (Variables|Default|GetfadeDelay))
    (Variables|Default|SetdialoguePlaying true)
    (UserInterface|Viewport|AddtoViewport _dialogueui 0)
    (Default|SpawnWidget _dialogueui)
    (Audio|PlaySound2D (Variables|Default|GetdialogueSound) 1.0 1.0 0.0 0 0))
  (|CallParentFunction))

(event EventPostStatesUpdate
  ;[1 1 1] First Encounter Updates
  (if (not (== (Variables|Default|GetstateIndex) 4))
    (if (Variables|Default|GetquestAccepted)
      (if (== (Variables|Default|GetstateIndex) 2)
        (Variables|Default|SetstateIndex 3))
      (elif (== (Variables|Default|GetstateIndex) 0)
        (Variables|Default|SetstateIndex 1)))
    (else
      (Actor|DestroyActor))))

(fn ConstructionScript
  (|CallParentFunction))