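; BP_NPC_TrashPaper is a quest dialogue NPC that tracks a sword through StateIndex and the QuestAccepted flag.
; Accepting the quest advances the state, resets the mesh rotation, destroys the trash-pile sword and shows the in-hand sword.
; On a post-state update with the quest accepted, it advances again, hides the in-hand sword and sets FinalSword on BP_NPC_MonkeyPirate, found by class lookup.
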(event Custom|Quest%20Accept%20Change
  (Variables|Default|SetquestAccepted true)
  (Variables|Default|SetstateIndex 1)
  (Transformation|SetRelativeRotation (Variables|Default|GetStaticMesh) "0, 0, 0" false false)
  (Actor|DestroyActor (Variables|Default|GettrashPileSword))
  (Rendering|SetVisibility (Variables|Default|GetInHandSword) true false))

(event EventPostStatesUpdate
  ;[1 1 1] First Encounter Updates
  (if (Variables|Default|GetquestAccepted)
    (Variables|Default|SetstateIndex 2)
    (bind _returnvalue (Actor|GetActorOfClass "/Game/Dialogue_Quests/NPC/BP_NPC_MonkeyPirate.BP_NPC_MonkeyPirate_C"))
    (Variables|/Game/Dialogue_Quests/NPC/BP_NPC_MonkeyPirate.BP_NPC_MonkeyPirate_C|SetfinalSword _returnvalue true)
    (Rendering|SetVisibility (Variables|Default|GetInHandSword) false false)))

(fn ConstructionScript
  (|CallParentFunction))