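; Monkey pirate quest NPC that takes collected swords from the player and inserts them before talking.
; PreStartDialogue banks collected swords and sets the dialogue state, then PlayAnimations plays unplayed sword sequences and delays dialogue until they finish.
; A final sword has its own state and longer sequence.
; Once the castle quest is complete, PostStatesUpdate advances dialogue states and notifies BP_NPC_TrashPaper after the required count is inserted.
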(event Custom|Add%20Sword
  ;[1 1 1] Add Sword
  (Math|Integer|IncrementInt (Variables|Default|GettotalCollected)))

(event Custom|Play%20Animations
  ;[1 1 1] Animations
  (if (Variables|Default|GetfinalSword)
    (Variables|Default|SetfinalSword false)
    (Sequencer|Player|Play (Variables|/Script/LevelSequence.LevelSequenceActor|GetSequencePlayer (Variables|Default|GetlastSword)) :!class /Script/MovieScene.MovieSceneSequencePlayer)
    (Variables|Default|SetplayingAnimation true)
    (Utilities|FlowControl|Delay 4.5)
    (Variables|Default|SetplayingAnimation false :!label _label)
    (CallFunction|StartDialogue)
    (elif (== (Variables|Default|GettotalInserted) 3)
      (Sequencer|Player|Play (Variables|/Script/LevelSequence.LevelSequenceActor|GetSequencePlayer (Variables|Default|GetthirdSword)) :!class /Script/MovieScene.MovieSceneSequencePlayer)
      (if (Variables|Default|GetsecondPlayed)
        _
        (else
          (Sequencer|Player|Play (Variables|/Script/LevelSequence.LevelSequenceActor|GetSequencePlayer (Variables|Default|GetsecondSword)) :!class /Script/MovieScene.MovieSceneSequencePlayer :!label _label_2)
          (Variables|Default|SetsecondPlayed true)
          (if (Variables|Default|GetfirstPlayed)
            _
            (else
              (Sequencer|Player|Play (Variables|/Script/LevelSequence.LevelSequenceActor|GetSequencePlayer (Variables|Default|GetfirstSword)) :!class /Script/MovieScene.MovieSceneSequencePlayer :!label _label_3)
              (Variables|Default|SetfirstPlayed true)))))
      (Variables|Default|SetplayingAnimation true)
      (Utilities|FlowControl|Delay 1.5)
      (goto _label)
      (elif (== (Variables|Default|GettotalInserted) 2)
        (goto _label_2)
        (elif (== (Variables|Default|GettotalInserted) 1)
          (goto _label_3))))))

(event Custom|Insert%20Sword
  ;[1 1 1] Insert Sword
  (if (not (Variables|Default|GetfinalSword))
    (Variables|Default|SettotalInserted (+ (Variables|Default|GettotalInserted) (Variables|Default|GettotalCollected)))
    (Variables|Default|SettotalCollected 0)
    (if (== (Variables|Default|GettotalInserted) (Variables|Default|GettotalNeeded))
      (Variables|Default|SetstateIndex 4)
      (else
        (Variables|Default|SetstateIndex 3)))
    (else
      (Variables|Default|SetstateIndex 6)))
  (CallFunction|PlayAnimations))

(event EventPreStartDialogue
  ;[1 1 1] Insert Sword Check
  (if (not (Variables|Default|GetplayingAnimation))
    (if (Variables|Default|GetfinalSword)
      (CallFunction|InsertSword :!label _label)
      (elif (> (Variables|Default|GettotalCollected) 0)
        (goto _label)
        (else
          (CallFunction|StartDialogue))))))

(event EventPostStatesUpdate
  ;[1 1 1] Quest Update Changes
  (if (Variables|Default|GetcastleQuestComplete)
    (if (== (Variables|Default|GetstateIndex) 1)
      (Variables|Default|SetstateIndex 2)
      (Variables|Default|SetquestAccepted true)
      (elif (and (== (Variables|Default|GetstateIndex) 3) (== (Variables|Default|GettotalCollected) 0))
        (Variables|Default|SetstateIndex 2)
        (elif (== (Variables|Default|GetstateIndex) 4)
          (Variables|Default|SetstateIndex 5)
          (bind _returnvalue (Actor|GetActorOfClass "/Game/Dialogue_Quests/NPC/BP_NPC_TrashPaper.BP_NPC_TrashPaper_C"))
          (Default|QuestAcceptChange _returnvalue)
          (elif (== (Variables|Default|GetstateIndex) 6)
            (Variables|Default|SetstateIndex 7)))))))

(fn ConstructionScript
  (|CallParentFunction))