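; Guard NPC that auto-starts dialogue when the player enters its initial collision and gates the princess and castle quests.
; PostStatesUpdate advances StateIndex and writes quest flags and states directly onto the Princess, then Monkey Pirate NPCs.
; The first step repositions its player-teleport point and dialogue camera and removes the initial collisions.
; Quest completion locks the player in dialogue during a fade while relocating the guards and tomato characters, swapping MrTomato for a static actor.
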(event OnComponentBeginOverlap(initialCollision)
  (params (OverlappedComponent :type Primitive%20Component%20Object%20Reference) (OtherActor :type Actor%20Object%20Reference) (OtherComp :type Primitive%20Component%20Object%20Reference) (OtherBodyIndex :type Integer) (bFromSweep :type Boolean) (SweepResult :type Hit%20Result%20Structure%20%28by%20ref%29))
  ;[1 1 1] Initial Auto Play Dialogue
  (Utilities|Casting|CastToBP_Player OtherActor)
  (CallFunction|EnterCollision))

(event EventPostStatesUpdate
  (bind _mrstomatomesh (Variables|Default|GetmrsTomatoMesh))
  ;[1 1 1] Start Princess Quest
  (if (== (Variables|Default|GetstateIndex) 0)
    (Variables|Default|SetstateIndex 1)
    (bind _returnvalue (Actor|GetActorOfClass "/Game/Dialogue_Quests/NPC/BP_NPC_Princess.BP_NPC_Princess_C"))
    (Variables|/Game/Dialogue_Quests/NPC/BP_NPC_Princess.BP_NPC_Princess_C|SetquestAccepted _returnvalue true)
    (Variables|/Game/Dialogue_Quests/NPC/BP_NPC.BP_NPC_C|SetstateIndex _returnvalue 2)
    (Transformation|SetRelativeLocation (Variables|Default|GetPlayerTeleport) (Variables|Default|GetnewPlayerLocation) false false)
    (Transformation|SetRelativeTransform (Variables|Default|GetCamera) (Variables|Default|GetnewCameraTransform) false false)
    (bind _initialcollision (Variables|Default|GetinitialCollision)
      (:then
        (bind _initialstandcollision (Variables|Default|GetinitialStandCollision)
          (:then
            (Components|DestroyComponent _initialcollision)
            (Components|DestroyComponent _initialstandcollision))
          (:else)))
      (:else))
    (else
      ;[1 1 1] Complete Quest + Activate Monkey Pirate Quest
      (if (== (Variables|Default|GetstateIndex) 2)
        (Variables|Default|SetstateIndex 3)
        (bind _returnvalue_2 (Actor|GetActorOfClass "/Game/Dialogue_Quests/NPC/BP_NPC_MonkeyPirate.BP_NPC_MonkeyPirate_C"))
        (Variables|/Game/Dialogue_Quests/NPC/BP_NPC_MonkeyPirate.BP_NPC_MonkeyPirate_C|SetcastleQuestComplete _returnvalue_2 true)
        (Variables|/Game/Dialogue_Quests/NPC/BP_NPC.BP_NPC_C|SetstateIndex _returnvalue_2 1)
        ;[1 1 1] Quest Finish Teleport
        (Variables|Default|SetdialogueStart true)
        (bind _returnvalue_3 (Actor|GetActorOfClass "/Game/PlayerCharacter/BP_Player.BP_Player_C"))
        (Variables|/Game/PlayerCharacter/BP_Player.BP_Player_C|SetinDialogue _returnvalue_3 true)
        (CallFunction|StartFade)
        (Utilities|FlowControl|Delay (Variables|Default|GetfadeDelay))
        (Transformation|SetActorRelativeLocation _mrstomatomesh (Transformation|GetWorldLocation (Variables|/Script/Engine.Actor|GetRootComponent (Variables|Default|GetmrsTomatoTP))))
        (Transformation|SetActorRotation _mrstomatomesh "0,90.000000, 0")
        (Transformation|SetActorRelativeLocation (Variables|Default|GetguardMesh) (Transformation|GetWorldLocation (Variables|/Script/Engine.Actor|GetRootComponent (Variables|Default|GetguardATP))))
        (bind _returnvalue_4 (Game|SpawnActorfromClass "/Game/Dialogue_Quests/Static_MrTomato.Static_MrTomato_C" (Variables|Default|GetSpawn%20Transform) "Undefined" 0 0))
        (Transformation|SetActorRelativeLocation _returnvalue_4 (Transformation|GetWorldLocation (Variables|/Script/Engine.Actor|GetRootComponent (Variables|Default|GetmrTomatoTP))))
        (Actor|DestroyActor (Variables|Default|GetmrTomatoNPC))
        (Transformation|SetActorLocation (Transformation|GetWorldLocation (Variables|/Script/Engine.Actor|GetRootComponent (Variables|Default|GetguardBTP))) false false)
        (Utilities|FlowControl|Delay (Variables|Default|GetfadeDelay))
        (Variables|Default|SetdialogueStart false)
        (bind _returnvalue_5 (Actor|GetActorOfClass "/Game/PlayerCharacter/BP_Player.BP_Player_C"))
        (Variables|/Game/PlayerCharacter/BP_Player.BP_Player_C|SetinDialogue _returnvalue_5 false)
        (CallFunction|ReactivateMovement)))))

(fn ConstructionScript
  (|CallParentFunction))