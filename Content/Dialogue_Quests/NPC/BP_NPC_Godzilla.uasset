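; Godzilla NPC Blueprint that runs a collection quest through dialogue states, extending parent NPC behavior.
; When dialogue starts while the MonkeyPirate NPC is at a specific state, the quest is accepted and StateIndex is set, then advanced after the first encounter.
; Quest updates count collected items and switch to the final state at the needed total, where movement no longer reactivates after dialogue.
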(event Custom|Quest%20Update
  ;[1 1 1] Quest Update
  (bind _result (Math|Integer|IncrementInt (Variables|Default|GettotalCollected))
    (:%20%20
      (if (== _result (Variables|Default|GettotalNeeded))
        (Variables|Default|SetstateIndex 3)))))

(event EventPreStartDialogue
  (bind _returnvalue (Actor|GetActorOfClass "/Game/Dialogue_Quests/NPC/BP_NPC_MonkeyPirate.BP_NPC_MonkeyPirate_C"))
  (if (not (== (Variables|/Game/Dialogue_Quests/NPC/BP_NPC.BP_NPC_C|GetstateIndex _returnvalue) 7))
    _
    (else
      (Variables|Default|SetquestAccepted true)
      (Variables|Default|SetstateIndex 1)))
  (|CallParentFunction))

(event EventReactivateMovement
  ;[1 1 1] End Dialogue
  (if (not (== (Variables|Default|GetstateIndex) 3))
    (|CallParentFunction)))

(event EventPostStatesUpdate
  ;[1 1 1] First Encounter Updates
  (if (Variables|Default|GetquestAccepted)
    (if (== (Variables|Default|GetstateIndex) 1)
      (Variables|Default|SetstateIndex 2))))

(fn ConstructionScript
  (|CallParentFunction))