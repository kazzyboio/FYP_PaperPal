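; Frog quest NPC whose collision and dialogue responses run only while BP_NPC_Princess is at state index 3.
; After its state update it advances the princess's quest, then locks the player in dialogue and starts a fade.
; During the fade it hides itself and spawns a Static_Frog at a target point.
; It overrides movement reactivation to do nothing, calling the parent version only after the swap, then destroys itself.
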(event EventReactivateMovement
  ;[1 1 1] Cancel Reactivate Movement
)

(event EventPostStatesUpdate
  ;[1 1 1] Update Princess Quest
  (bind _returnvalue (Actor|GetActorOfClass "/Game/Dialogue_Quests/NPC/BP_NPC_Princess.BP_NPC_Princess_C"))
  (Default|QuestUpdate _returnvalue)
  (Variables|Default|SetdialogueStart true)
  (bind _returnvalue_2 (Actor|GetActorOfClass "/Game/PlayerCharacter/BP_Player.BP_Player_C"))
  (Variables|/Game/PlayerCharacter/BP_Player.BP_Player_C|SetinDialogue _returnvalue_2 true)
  (CallFunction|StartFade)
  (Utilities|FlowControl|Delay (Variables|Default|GetfadeDelay))
  (Rendering|SetActorHiddenInGame true)
  (bind _returnvalue_3 (Game|SpawnActorfromClass "/Game/Dialogue_Quests/Static_Frog.Static_Frog_C" (Variables|Default|GetSpawn%20Transform) "Undefined" 0 0))
  (Transformation|SetActorRelativeLocation _returnvalue_3 (Transformation|GetWorldLocation (Variables|/Script/Engine.Actor|GetRootComponent (Variables|Default|GettargetPoint))))
  (Utilities|FlowControl|Delay (Variables|Default|GetfadeDelay))
  (|CallParentFunction)
  (Variables|Default|SetdialogueStart false)
  (bind _returnvalue_4 (Actor|GetActorOfClass "/Game/PlayerCharacter/BP_Player.BP_Player_C"))
  (Variables|/Game/PlayerCharacter/BP_Player.BP_Player_C|SetinDialogue _returnvalue_4 false)
  (Actor|DestroyActor))

(event EventActivateDialogue
  ;[1 1 1] Check Quest Accepted
  (bind _returnvalue (Actor|GetActorOfClass "/Game/Dialogue_Quests/NPC/BP_NPC_Princess.BP_NPC_Princess_C"))
  (if (== (Variables|/Game/Dialogue_Quests/NPC/BP_NPC.BP_NPC_C|GetstateIndex _returnvalue) 3)
    (|CallParentFunction)))

(event EventEnterCollision
  ;[1 1 1] Check Quest Accepted
  (bind _returnvalue (Actor|GetActorOfClass "/Game/Dialogue_Quests/NPC/BP_NPC_Princess.BP_NPC_Princess_C"))
  (if (== (Variables|/Game/Dialogue_Quests/NPC/BP_NPC.BP_NPC_C|GetstateIndex _returnvalue) 3)
    (|CallParentFunction)))

(event EventExitCollision
  ;[1 1 1] Check Quest Accepted
  (bind _returnvalue (Actor|GetActorOfClass "/Game/Dialogue_Quests/NPC/BP_NPC_Princess.BP_NPC_Princess_C"))
  (if (== (Variables|/Game/Dialogue_Quests/NPC/BP_NPC.BP_NPC_C|GetstateIndex _returnvalue) 3)
    (|CallParentFunction)))

(fn ConstructionScript
  (|CallParentFunction))