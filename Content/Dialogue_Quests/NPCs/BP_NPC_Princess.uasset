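; Princess NPC, a dialogue and quest character whose logic branches on RowName between a Castle variant and a Party variant.
; In the Castle, collecting all quest items moves her to a finishing state whose dialogue fades out, swaps her for a static princess at a target point and updates the guards.
; At the Party, her state follows Mrs Tomato Head's progress before each conversation, finally adding a guest to the Monkey Pirate.
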(event Custom|Quest%20Update
  ;[1 1 1] Quest Update
  (if (== (Variables|Default|GetRow%20Name) "Princess_Castle")
    (bind _result (Math|Integer|IncrementInt (Variables|Default|GettotalCollected))
      (:%20%20
        (if (== _result (Variables|Default|GettotalNeeded))
          (Variables|Default|SetstateIndex 4))))))

(event EventDialogueEvent
  (bind _dialogueui (Variables|Default|GetdialogueUI))
  ;[1 1 1] Quest Finish Teleport
  (if (== (Variables|Default|GetRow%20Name) "Princess_Castle")
    (if (and (== (Variables|Default|GetstateIndex) 4) (== (Variables|Default|GetdialogueIndex) 2))
      (Variables|Default|SetdialoguePlaying false)
      (Default|DespawnWidget (Variables|Default|GetdialogueUI))
      (CallFunction|StartFade)
      (Utilities|FlowControl|Delay (Variables|Default|GetfadeDelay))
      (Rendering|SetActorHiddenInGame true)
      (bind _returnvalue (Game|SpawnActorfromClass "/Game/Dialogue_Quests/Static_Princess.Static_Princess_C" (Variables|Default|GetSpawn%20Transform) "Undefined" 0 0))
      (Transformation|SetActorRelativeLocation _returnvalue (Transformation|GetWorldLocation (Variables|/Script/Engine.Actor|GetRootComponent (Variables|Default|GettargetPoint))))
      (bind _returnvalue_2 (Actor|GetActorOfClass "/Game/Dialogue_Quests/NPCs/BP_NPC_Guards.BP_NPC_Guards_C"))
      (Variables|/Game/Dialogue_Quests/NPCs/BP_NPC.BP_NPC_C|SetstateIndex _returnvalue_2 2)
      (Utilities|FlowControl|Delay (Variables|Default|GetfadeDelay))
      (Variables|Default|SetdialoguePlaying true)
      (UserInterface|Viewport|AddtoViewport _dialogueui 0)
      (Default|SpawnWidget _dialogueui)
      (Audio|PlaySound2D (Variables|Default|GetdialogueSound) 1.0 1.0 0.0 0 0)))
  (|CallParentFunction))

(event EventPreStartDialogue
  ;[1 1 1] Check for Mrs Tomato Updates
  (if (== (Variables|Default|GetRow%20Name) "Princess_Party")
    (bind _returnvalue (Actor|GetActorOfClass "/Game/Dialogue_Quests/NPCs/BP_NPC_MrsTomatoHead.BP_NPC_MrsTomatoHead_C"))
    (if (and (== (Variables|/Game/Dialogue_Quests/NPCs/BP_NPC.BP_NPC_C|GetstateIndex _returnvalue) 2) (== (Variables|Default|GetstateIndex) 1))
      (Variables|Default|SetstateIndex 2)
      (elif (and (== (Variables|/Game/Dialogue_Quests/NPCs/BP_NPC.BP_NPC_C|GetstateIndex _returnvalue) 4) (== (Variables|Default|GetstateIndex) 3))
        (Variables|Default|SetstateIndex 4))))
  (|CallParentFunction))

(event EventPostStatesUpdate
  ;[1 1 1] Post States Update (Castle)
  (if (== (Variables|Default|GetRow%20Name) "Princess_Castle")
    (if (!= (Variables|Default|GetstateIndex) 4)
      (if (Variables|Default|GetquestAccepted)
        (if (== (Variables|Default|GetstateIndex) 2)
          (Variables|Default|SetstateIndex 3))
        (elif (== (Variables|Default|GetstateIndex) 0)
          (Variables|Default|SetstateIndex 1)))
      (else
        (Actor|DestroyActor)))
    (else
      ;[1 1 1] Post States Update (Party)
      (if (== (Variables|Default|GetstateIndex) 0)
        (Variables|Default|SetstateIndex 1)
        (elif (== (Variables|Default|GetstateIndex) 2)
          (Variables|Default|SetstateIndex 3)
          (elif (== (Variables|Default|GetstateIndex) 4)
            (Variables|Default|SetstateIndex 5)
            (bind _returnvalue (Actor|GetActorOfClass "/Game/Dialogue_Quests/NPCs/BP_NPC_MonkeyPirate.BP_NPC_MonkeyPirate_C"))
            (Default|AddGuest _returnvalue)))))))

(fn ConstructionScript
  (|CallParentFunction))