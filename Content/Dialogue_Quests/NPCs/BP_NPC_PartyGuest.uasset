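; BP_NPC_PartyGuest is a dialogue NPC for a party guest that can be spawned into the scene on demand.
; SpawnGuests moves the actor and its ExtraMeshes down by a fixed Z offset and unhides them, restoring capsule and sphere collision profiles on the guest.
; PreStartDialogue sets StateIndex to 0 before calling the parent, as the random quote branch is disconnected.
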(event Custom|Spawn%20Guests
  (Transformation|SetActorLocation (+ (Transformation|GetActorLocation) "0,0,-3553.000000") false false)
  (Collision|SetCollisionProfileName (Variables|Default|GetCapsuleComponent) "BlockAllDynamic" true :!class /Script/Engine.PrimitiveComponent)
  (Collision|SetCollisionProfileName (Variables|Default|GetSphereCollision) "OverlapAllDynamic" true :!class /Script/Engine.PrimitiveComponent)
  (Rendering|SetActorHiddenInGame false)
  (for _array_element (Variables|Default|GetextraMeshes)
    (Rendering|SetActorHiddenInGame _array_element false)
    (Transformation|SetActorLocation _array_element (+ (Transformation|GetActorLocation _array_element) "0,0,-3553.000000") false false)))

(event EventPreStartDialogue
  ;[1 1 1] Random Select Quote
  (Variables|Default|SetstateIndex 0)
  (|CallParentFunction))

(fn ConstructionScript
  (|CallParentFunction))