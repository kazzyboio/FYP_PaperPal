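; BP_NPC_SelfDialogue is an NPC dialogue variant for the player's self-dialogue, with the speaker set to the player's name.
; Collision calls PlayerAdjustments after a short delay, and the activation override skips the stinky check.
; The start row blends the view to a camera actor before the parent pan, then shows an input-device-specific movement tutorial after the state update.
; The stinky pickup row calls Stinky, and the actor destroys itself afterwards.
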(event EventActivateDialogue
  ;[1 1 1] No Stinky Check for Self Dialogue
  (if (not (Variables|Default|GetdialogueStart))
    (CallFunction|PlayerAdjustments)))

(event EventPostStatesUpdate
  ;[1 1 1] Post States Events
  (if (== (Variables|Default|GetRow%20Name) "Self_Dialogue_Start")
    (bind _asbp_player (Utilities|Casting|CastToBP_Player (Game|GetPlayerCharacter 0)))
    (switch Utilities|FlowControl|Switch|SwitchonInputDevice (Variables|/Game/PlayerCharacter/BP_Player.BP_Player_C|GetCurrentInputDevice _asbp_player)
      (:NewEnumerator0
        (bind _returnvalue (UserInterface|CreateWidget "/Game/Assets/UI/WB/WB_Tutorial.WB_Tutorial_C"))
        (UserInterface|Viewport|AddtoViewport _returnvalue 0)
        (Default|MoveTutorialAnimationKBM _returnvalue))
      (:NewEnumerator1
        (bind _returnvalue_2 (UserInterface|CreateWidget "/Game/Assets/UI/WB/WB_Tutorial.WB_Tutorial_C"))
        (UserInterface|Viewport|AddtoViewport _returnvalue_2 0)
        (Default|MoveTutorialAniPad _returnvalue_2)))
    (elif (== (Variables|Default|GetRow%20Name) "Self_Dialogue_Stinky_Pickup")
      (CallFunction|Stinky)))
  (Actor|DestroyActor))

(event EventCameraPan
  (bind _blendtime (Variables|Default|GetblendTime))
  ;[1 1 1] Camera Pan
  (if (== (Variables|Default|GetRow%20Name) "Self_Dialogue_Start")
    (Game|Player|SetViewTargetwithBlend (Game|GetPlayerController 0) (Variables|Default|GetcameraActor) _blendtime "VTBlend_Linear" 0.0 false)
    (Utilities|FlowControl|Delay (+ _blendtime (Variables|Default|GetcameraStayTime))))
  (|CallParentFunction))

(event EventEnterCollision
  ;[1 1 1] Collision Event
  (Utilities|FlowControl|Delay 0.2)
  (CallFunction|PlayerAdjustments))

(fn ConstructionScript
  (|CallParentFunction)
  (Variables|Default|SetcurrentSpeaker (Variables|Default|GetplayerName)))