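; Guards NPC that starts and completes the Princess quest, then activates the Monkey Pirate quest.
; Overrides parent NPC dialogue hooks, using StateIndex to update other quest NPCs, auto-play collision, player teleport and camera pans.
; Fade-masked teleports restage the guards and Mr and Mrs Tomato for their reunion.
; Quest completion also swaps Mr Tomato's NPC for a static actor and updates highlight meshes.
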(event OnComponentBeginOverlap(initialCollision)
  (params (OverlappedComponent :type Primitive%20Component%20Object%20Reference) (OtherActor :type Actor%20Object%20Reference) (OtherComp :type Primitive%20Component%20Object%20Reference) (OtherBodyIndex :type Integer) (bFromSweep :type Boolean) (SweepResult :type Hit%20Result%20Structure%20%28by%20ref%29))
  ;[1 1 1] Initial Auto Play Dialogue
  (Utilities|Casting|CastToBP_Player OtherActor)
  (CallFunction|EnterCollision))

(event EventCameraPan
  (bind _blendtime (Variables|Default|GetblendTime))
  ;[1 1 1] Camera Pan
  (if (== (Variables|Default|GetstateIndex) 2)
    (Game|Player|SetViewTargetwithBlend (Game|GetPlayerController 0) (Variables|Default|GetcameraActorA) (Variables|Default|GetblendTime) "VTBlend_Linear" 0.0 false)
    (Utilities|FlowControl|Delay (+ _blendtime (Variables|Default|GetcameraStayTime)) :!label _label)
    (elif (== (Variables|Default|GetstateIndex) 3)
      (Game|Player|SetViewTargetwithBlend (Game|GetPlayerController 0) (Variables|Default|GetcameraActorB) _blendtime "VTBlend_Linear" 0.0 false)
      (goto _label)
      (else
        _)))
  (|CallParentFunction))

(event EventReactivateMovement
  ;[1 1 1] Lock Movement for Fade
  (if (!= (Variables|Default|GetstateIndex) 2)
    (|CallParentFunction)))

(event EventPostStatesUpdate
  (bind _mrstomatomesh (Variables|Default|GetmrsTomatoMesh))
  ;[1 1 1] Start Princess Quest
  (if (== (Variables|Default|GetstateIndex) 0)
    (Variables|Default|SetstateIndex 1)
    (bind _returnvalue (Actor|GetActorOfClass "/Game/Dialogue_Quests/NPCs/BP_NPC_MrTomatoHead.BP_NPC_MrTomatoHead_C"))
    (Components|Sphere|SetSphereRadius (Variables|/Game/Dialogue_Quests/NPCs/BP_NPC.BP_NPC_C|GetSphereCollision _returnvalue) 2e+02 true)
    (bind _returnvalue_2 (Actor|GetActorOfClass "/Game/Dialogue_Quests/NPCs/BP_NPC_Princess.BP_NPC_Princess_C"))
    (Variables|/Game/Dialogue_Quests/NPCs/BP_NPC_Princess.BP_NPC_Princess_C|SetquestAccepted _returnvalue_2 true)
    (Variables|/Game/Dialogue_Quests/NPCs/BP_NPC.BP_NPC_C|SetstateIndex _returnvalue_2 2)
    (Transformation|SetRelativeLocation (Variables|Default|GetPlayerTeleport) (Variables|Default|GetnewPlayerLocation) false false)
    (Transformation|SetRelativeTransform (Variables|Default|GetCamera) (Variables|Default|GetnewCameraTransform) false false)
    (bind _initialcollision (Variables|Default|GetinitialCollision)
      (:then
        (bind _initialstandcollision (Variables|Default|GetinitialStandCollision)
          (:then
            (Components|DestroyComponent _initialcollision)
            (Components|DestroyComponent _initialstandcollision))
          (:else)))
      (:else))
    (else
      ;[1 1 1] Complete Quest + Activate Monkey Pirate Quest
      (if (== (Variables|Default|GetstateIndex) 2)
        (Variables|Default|SetstateIndex 3)
        (Transformation|SetRelativeLocation (Variables|Default|GetPlayerTeleport) (Variables|Default|GetnewPlayerLocation2) false false)
        (bind _returnvalue_3 (Actor|GetActorOfClass "/Game/Dialogue_Quests/NPCs/BP_NPC_MonkeyPirate.BP_NPC_MonkeyPirate_C"))
        (Variables|/Game/Dialogue_Quests/NPCs/BP_NPC_MonkeyPirate.BP_NPC_MonkeyPirate_C|SetcastleQuestComplete _returnvalue_3 true)
        (Variables|/Game/Dialogue_Quests/NPCs/BP_NPC.BP_NPC_C|SetstateIndex _returnvalue_3 1)
        ;[1 1 1] Quest Finish Teleport
        (Variables|Default|SetdialogueStart true)
        (bind _returnvalue_4 (Actor|GetActorOfClass "/Game/PlayerCharacter/BP_Player.BP_Player_C"))
        (Variables|/Game/PlayerCharacter/BP_Player.BP_Player_C|SetinDialogue _returnvalue_4 true)
        (CallFunction|StartFade)
        (Utilities|FlowControl|Delay (Variables|Default|GetfadeDelay))
        (Transformation|SetActorLocation _mrstomatomesh (Transformation|GetWorldLocation (Variables|/Script/Engine.Actor|GetRootComponent (Variables|Default|GetmrsTomatoTP2))) false false)
        (Transformation|SetActorRotation _mrstomatomesh "0,90.000000, 0")
        (bind _returnvalue_5 (Game|SpawnActorfromClass "/Game/Dialogue_Quests/StaticActors/Static_MrTomato.Static_MrTomato_C" (Variables|Default|GetSpawn%20Transform) "Undefined" 0 0))
        (Transformation|SetActorLocation _returnvalue_5 (Transformation|GetWorldLocation (Variables|/Script/Engine.Actor|GetRootComponent (Variables|Default|GetmrTomatoTP2))) false false)
        (Actor|DestroyActor (Variables|Default|GetmrTomatoNPC))
        (Transformation|SetActorLocation (Transformation|GetWorldLocation (Variables|/Script/Engine.Actor|GetRootComponent (Variables|Default|GetguardBTP))) false false)
        (Transformation|SetRelativeLocation (Variables|Default|GetStaticMesh) "0, 0,-54.000000" false false)
        ;[1 1 1] Change Highlight Actors
        (Utilities|Array|RemoveIndex (Variables|Default|GetextraMeshes) 1)
        (bind _returnvalue_6 (Actor|GetActorOfClass "/Game/Dialogue_Quests/StaticActors/Static_Princess.Static_Princess_C"))
        (Utilities|Array|Add (Variables|Default|GetextraMeshes) _returnvalue_6)
        (bind _returnvalue_7 (Actor|GetActorOfClass "/Game/Dialogue_Quests/NPCs/BP_NPC_MonkeyPirate.BP_NPC_MonkeyPirate_C"))
        (bind _returnvalue_8 (Actor|GetActorOfClass "/Game/Dialogue_Quests/StaticActors/Static_MrTomato.Static_MrTomato_C"))
        (Utilities|Array|Add (Variables|/Game/Dialogue_Quests/NPCs/BP_NPC.BP_NPC_C|GetextraMeshes _returnvalue_7) _returnvalue_8)
        (bind _returnvalue_9 (Actor|GetActorOfClass "/Game/Dialogue_Quests/StaticActors/Static_MrsTomato.Static_MrsTomato_C"))
        (Utilities|Array|Add (Variables|/Game/Dialogue_Quests/NPCs/BP_NPC.BP_NPC_C|GetextraMeshes _returnvalue_7) _returnvalue_9)
        (Utilities|FlowControl|Delay (Variables|Default|GetfadeDelay))
        (Variables|Default|SetdialogueStart false)
        (bind _returnvalue_10 (Actor|GetActorOfClass "/Game/PlayerCharacter/BP_Player.BP_Player_C"))
        (Variables|/Game/PlayerCharacter/BP_Player.BP_Player_C|SetinDialogue _returnvalue_10 false)
        (|CallParentFunction)))))

(event EventDialogueEvent
  (bind _mrtomatonpc (Variables|Default|GetmrTomatoNPC))
  (bind _dialogueui (Variables|Default|GetdialogueUI))
  (bind _mrstomatomesh (Variables|Default|GetmrsTomatoMesh))
  ;[1 1 1] Mr and Mrs Tomato Reunite Fade Event
  (if (and (== 2 (Variables|Default|GetstateIndex)) (== 7 (Variables|Default|GetdialogueIndex)))
    (Variables|Default|SetdialoguePlaying false)
    (Default|DespawnWidget (Variables|Default|GetdialogueUI))
    (CallFunction|StartFade)
    (Utilities|FlowControl|Delay (Variables|Default|GetfadeDelay))
    (Transformation|SetActorLocation (Variables|Default|GetguardMesh) (Transformation|GetWorldLocation (Variables|/Script/Engine.Actor|GetRootComponent (Variables|Default|GetguardATP))) false false)
    (Transformation|SetWorldLocation (Variables|Default|GetStaticMesh) (Transformation|GetWorldLocation (Variables|/Script/Engine.Actor|GetRootComponent (Variables|Default|GetguardBTP))) false false)
    (Transformation|SetActorLocation _mrstomatomesh (Transformation|GetWorldLocation (Variables|/Script/Engine.Actor|GetRootComponent (Variables|Default|GetmrsTomatoTP1))) false false)
    (Transformation|SetActorRotation _mrstomatomesh "0,135.000000, 0")
    (Transformation|SetActorLocation _mrtomatonpc (Transformation|GetWorldLocation (Variables|/Script/Engine.Actor|GetRootComponent (Variables|Default|GetmrTomatoTP1))) false false)
    (Transformation|SetActorRotation _mrtomatonpc "0,225.000000, 0")
    (Utilities|FlowControl|Delay (Variables|Default|GetfadeDelay))
    (Variables|Default|SetdialoguePlaying true)
    (UserInterface|Viewport|AddtoViewport _dialogueui 0)
    (Default|SpawnWidget _dialogueui)
    (Audio|PlaySound2D (Variables|Default|GettypeSoundA) 1.0 1.0 0.0 0 0))
  (|CallParentFunction))

(event EventPreStartDialogue
  ;[1 1 1] Check for Monkey Pirate (Where's Jerry)
  (bind _returnvalue (Actor|GetActorOfClass "/Game/Dialogue_Quests/NPCs/BP_NPC_MonkeyPirate.BP_NPC_MonkeyPirate_C"))
  (if (and (Variables|/Game/Dialogue_Quests/NPCs/BP_NPC_MonkeyPirate.BP_NPC_MonkeyPirate_C|GetpartyQuestAccepted _returnvalue) (== (Variables|Default|GetstateIndex) 3))
    (Variables|Default|SetstateIndex 4))
  (|CallParentFunction))

(fn ConstructionScript
  (|CallParentFunction))