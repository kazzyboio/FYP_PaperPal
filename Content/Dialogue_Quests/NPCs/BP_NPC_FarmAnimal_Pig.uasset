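; Pig NPC dialogue Blueprint that links the Mr Tomato Head key quest and the Farmer quest.
; Parent dialogue hooks drive a StateIndex machine, advanced by looking up both quest givers' accepted flags.
; A dialogue line pauses the UI, blends to a cutscene camera and spawns the tomato key.
; Afterwards, if the Farmer quest is accepted, it updates the Farmer, fades and moves the pig to a target point.
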(event Custom|Quest%20Update
  ;[1 1 1] Update Pig Quest
)

(event EventDialogueEvent
  (bind _blendtime (Variables|Default|GetblendTime))
  (bind _dialogueui (Variables|Default|GetdialogueUI))
  (bind _blendtime_2 (Variables|Default|GetblendTime))
  (if (and (== 3 (Variables|Default|GetstateIndex)) (== 2 (Variables|Default|GetdialogueIndex)))
    (Variables|Default|SetdialoguePlaying false)
    (Default|DespawnWidget (Variables|Default|GetdialogueUI))
    (Game|Player|SetViewTargetwithBlend (Game|GetPlayerController 0) (Variables|Default|GetcameraActor) _blendtime "VTBlend_Cubic" 0.0 false)
    (Utilities|FlowControl|Delay (+ _blendtime (Variables|Default|GetcameraStayTime)))
    (bind _returnvalue (Game|SpawnActorfromClass "/Game/Dialogue_Quests/BP_QuestItem_TomatoKey.BP_QuestItem_TomatoKey_C" (Variables|Default|GetSpawn%20Transform) "Undefined" 0 0))
    (Transformation|SetActorRelativeLocation _returnvalue (Transformation|GetWorldLocation (Variables|/Script/Engine.Actor|GetRootComponent (Variables|Default|GetkeyTargetPoint))))
    (Game|Player|SetViewTargetwithBlend (Game|GetPlayerController 0) (Components|GetOwner (Variables|Default|GetCamera)) _blendtime_2 "VTBlend_Cubic" 0.0 false)
    (Utilities|FlowControl|Delay _blendtime_2)
    (Variables|Default|SetdialoguePlaying true)
    (UserInterface|Viewport|AddtoViewport _dialogueui 0)
    (Default|SpawnWidget _dialogueui)
    (Audio|PlaySound2D (Variables|Default|GetdialogueSound) 1.0 1.0 0.0 0 0))
  (|CallParentFunction))

(event EventPreStartDialogue
  ;[1 1 1] Check for Farmer / Mr Tomato Quest Acceptance
  (if (== (Variables|Default|GetstateIndex) 0)
    (bind _returnvalue (Actor|GetActorOfClass "/Game/Dialogue_Quests/NPCs/BP_NPC_MrTomatoHead.BP_NPC_MrTomatoHead_C"))
    (if (Variables|/Game/Dialogue_Quests/NPCs/BP_NPC_MrTomatoHead.BP_NPC_MrTomatoHead_C|GetkeyQuestAccepted _returnvalue)
      (bind _returnvalue_2 (Actor|GetActorOfClass "/Game/Dialogue_Quests/NPCs/BP_NPC_Farmer.BP_NPC_Farmer_C"))
      (if (Variables|/Game/Dialogue_Quests/NPCs/BP_NPC_Farmer.BP_NPC_Farmer_C|GetquestAccepted _returnvalue_2)
        (Variables|Default|SetstateIndex 1)
        (else
          (Variables|Default|SetstateIndex 1)))
      (else
        (bind _returnvalue_3 (Actor|GetActorOfClass "/Game/Dialogue_Quests/NPCs/BP_NPC_Farmer.BP_NPC_Farmer_C"))
        (if (Variables|/Game/Dialogue_Quests/NPCs/BP_NPC_Farmer.BP_NPC_Farmer_C|GetquestAccepted _returnvalue_3)
          (Variables|Default|SetstateIndex 1))))
    (elif (== (Variables|Default|GetstateIndex) 4)
      (bind _returnvalue_4 (Actor|GetActorOfClass "/Game/Dialogue_Quests/NPCs/BP_NPC_Farmer.BP_NPC_Farmer_C"))
      (if (Variables|/Game/Dialogue_Quests/NPCs/BP_NPC_Farmer.BP_NPC_Farmer_C|GetquestAccepted _returnvalue_4)
        (Variables|Default|SetstateIndex 5))))
  (|CallParentFunction))

(event EventPostStatesUpdate
  ;[1 1 1] Post State Updates
  (if (or (== (Variables|Default|GetstateIndex) 1) (or (== (Variables|Default|GetstateIndex) 1) (== (Variables|Default|GetstateIndex) 1)))
    (Variables|Default|SetquestAccepted true)
    (Variables|Default|SetstateIndex 2)
    (elif (== (Variables|Default|GetstateIndex) 2)
      (Variables|Default|SetstateIndex 3)
      (elif (== (Variables|Default|GetstateIndex) 3)
        (bind _returnvalue (Actor|GetActorOfClass "/Game/Dialogue_Quests/NPCs/BP_NPC_Farmer.BP_NPC_Farmer_C"))
        (if (Variables|/Game/Dialogue_Quests/NPCs/BP_NPC_Farmer.BP_NPC_Farmer_C|GetquestAccepted _returnvalue)
          (Default|QuestUpdate _returnvalue)
          (Variables|Default|SetdialoguePlaying false :!label _label)
          (Default|DespawnWidget (Variables|Default|GetdialogueUI))
          (CallFunction|StartFade)
          (Utilities|FlowControl|Delay (Variables|Default|GetfadeDelay))
          (Transformation|SetActorLocation (Transformation|GetWorldLocation (Variables|/Script/Engine.Actor|GetRootComponent (Variables|Default|GetpigTargetPoint))) false false)
          (Variables|Default|SetstateIndex 6)
          (else
            (Variables|Default|SetstateIndex 4)))
        (elif (== (Variables|Default|GetstateIndex) 5)
          (bind _returnvalue_2 (Actor|GetActorOfClass "/Game/Dialogue_Quests/NPCs/BP_NPC_Farmer.BP_NPC_Farmer_C"))
          (Default|QuestUpdate _returnvalue_2)
          (goto _label))))))

(fn ConstructionScript
  (|CallParentFunction))