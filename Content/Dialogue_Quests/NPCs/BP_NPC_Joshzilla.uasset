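; Joshzilla quest NPC, a dialogue child that runs a building-block collection side quest tied to the Monkey Pirate's party quest.
; Accepting the party quest unhides physics blocks and enables auto-activation; StateIndex then steers dialogue through intro, collection and completion.
; Construction counts BP_Block actors as the target; reaching it leads to a fade that swaps small blocks for BP_BigBlock with a camera blend.
; Finishing adds a party guest and updates the journal.
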(event Custom|Quest%20Update
  ;[1 1 1] Quest Update
  (bind _result (Math|Integer|IncrementInt (Variables|Default|GettotalCollected))
    (:%20%20
      (if (== _result (Variables|Default|GettotalNeeded))
        (Variables|Default|SetstateIndex 3)
        (Utilities|FlowControl|Delay 1.0)
        (CallFunction|PlayerAdjustments)))))

(event Custom|AutoDialogue
  ;[1 1 1] Auto Dialogue
  (Components|Activation|Deactivate (Variables|/Script/Engine.Character|GetCharacterMovement (Game|GetPlayerCharacter 0)))
  (Rendering|SetRenderCustomDepth (Variables|Character|GetMesh) false)
  (bind _returnvalue (Actor|GetActorOfClass "/Game/PlayerCharacter/BP_Player.BP_Player_C"))
  (Default|HIDEUI (Variables|/Game/PlayerCharacter/BP_Player.BP_Player_C|GetPOP%20up _returnvalue))
  (Rendering|SetVisibility (Variables|/Game/PlayerCharacter/BP_Player.BP_Player_C|GetNS_Jump _returnvalue) false false)
  (Default|DisablePlane _returnvalue)
  (Default|StopSprint _returnvalue)
  (Components|Animation|PlayAnimation (Variables|/Script/Engine.Character|GetMesh _returnvalue) "/Game/PlayerCharacter/NewCHara/Anim_PlayerIdle.Anim_PlayerIdle" true)
  (Utilities|FlowControl|Delay 3.5)
  (Variables|Default|SetstateIndex 5)
  (CallFunction|PlayerAdjustments))

(event EventDialogueEvent
  (bind _blendtime (Variables|Default|GetblendTime))
  (bind _dialogueui (Variables|Default|GetdialogueUI))
  ;[1 1 1] Fade, Remove Small Blocks, Spawn and Pan to Big Block
  (if (and (== 3 (Variables|Default|GetstateIndex)) (== 3 (Variables|Default|GetdialogueIndex)))
    (Variables|Default|SetdialoguePlaying false)
    (Default|DespawnWidget (Variables|Default|GetdialogueUI))
    (CallFunction|StartFade)
    (Utilities|FlowControl|Delay (Variables|Default|GetfadeDelay))
    (bind _returnvalue (Actor|GetActorOfClass "/Game/BPActors/BP_BigBlock.BP_BigBlock_C"))
    (Default|Spawn _returnvalue)
    (bind _outactors (Actor|GetAllActorswithTag "BuildingBlock"))
    (Actor|DestroyActor _outactors)
    (bind _outactors_2 (Actor|GetAllActorsOfClass "/Game/BPActors/BP_Block.BP_Block_C"))
    (Actor|DestroyActor _outactors_2)
    (Utilities|FlowControl|Delay (Variables|Default|GetfadeDelay))
    (Game|Player|SetViewTargetwithBlend (Game|GetPlayerController 0) (Variables|Default|GetcameraActor) _blendtime "VTBlend_Cubic" 0.0 false)
    (Utilities|FlowControl|Delay (+ _blendtime (Variables|Default|GetcameraStayTime)))
    (Variables|Default|SetdialoguePlaying true)
    (UserInterface|Viewport|AddtoViewport _dialogueui 0)
    (Default|SpawnWidget _dialogueui)
    (Audio|PlaySound2D (Variables|Default|GettypeSoundA) 1.0 1.0 0.0 0 0))
  (|CallParentFunction))

(event EventPreStartDialogue
  ;[1 1 1] Quest Accept Check
  (bind _returnvalue (Actor|GetActorOfClass "/Game/Dialogue_Quests/NPCs/BP_NPC_MonkeyPirate.BP_NPC_MonkeyPirate_C"))
  (if (and (Variables|/Game/Dialogue_Quests/NPCs/BP_NPC_MonkeyPirate.BP_NPC_MonkeyPirate_C|GetpartyQuestAccepted _returnvalue) (not (Variables|Default|GetquestAccepted)))
    (Variables|Default|SetstateIndex 1))
  (|CallParentFunction))

(event EventPostStatesUpdate
  ;[1 1 1] First Encounter Updates
  (bind _returnvalue (Actor|GetActorOfClass "/Game/Dialogue_Quests/NPCs/BP_NPC_MonkeyPirate.BP_NPC_MonkeyPirate_C"))
  (if (Variables|/Game/Dialogue_Quests/NPCs/BP_NPC_MonkeyPirate.BP_NPC_MonkeyPirate_C|GetpartyQuestAccepted _returnvalue)
    (if (== (Variables|Default|GetstateIndex) 1)
      (Variables|Default|SetstateIndex 2)
      (Variables|Default|SetquestAccepted true)
      (Variables|Default|SetautoActivate false)
      (Components|Sphere|SetSphereRadius (Variables|Default|GetSphereCollision) 2.5e+02 true)
      (elif (== (Variables|Default|GetstateIndex) 3)
        (Variables|Default|SetstateIndex 4)
        (elif (== (Variables|Default|GetstateIndex) 5)
          (Variables|Default|SetstateIndex 6)
          (bind _returnvalue_2 (Actor|GetActorOfClass "/Game/Dialogue_Quests/NPCs/BP_NPC_MonkeyPirate.BP_NPC_MonkeyPirate_C"))
          (Default|AddGuest _returnvalue_2)
          (bind _returnvalue_3 (Actor|GetActorOfClass "/Game/PlayerCharacter/BP_Player.BP_Player_C"))
          (Default|JoshzillaDone (Variables|/Game/PlayerCharacter/BP_Player.BP_Player_C|GetJournalUI _returnvalue_3)))))))

(event EventTick
  (params (DeltaSeconds :type Float%20%28single-precision%29))
  ;[1 1 1] Post Monkey Pirate Changes
  (bind _returnvalue (Actor|GetActorOfClass "/Game/Dialogue_Quests/NPCs/BP_NPC_MonkeyPirate.BP_NPC_MonkeyPirate_C"))
  (if (and (Variables|Default|GetblockSpawn) (Variables|/Game/Dialogue_Quests/NPCs/BP_NPC_MonkeyPirate.BP_NPC_MonkeyPirate_C|GetpartyQuestAccepted _returnvalue))
    (bind _outactors (Actor|GetAllActorswithTag "BuildingBlock"))
    (for _array_element _outactors
      (Rendering|SetActorHiddenInGame _array_element false)
      (Physics|SetSimulatePhysics (Actor|GetComponentbyClass _array_element "/Script/Engine.StaticMeshComponent") true)
      (Collision|SetCollisionProfileName (Actor|GetComponentbyClass _array_element "/Script/Engine.StaticMeshComponent") "PhysicsActor" true :!class /Script/Engine.PrimitiveComponent))
    (Actor|DestroyActor (Variables|Default|GetblockPile))
    (Components|Sphere|SetSphereRadius (Variables|Default|GetSphereCollision) 4e+02 true)
    (Variables|Default|SetautoActivate true)
    (Variables|Default|SetblockSpawn false)))

(fn ConstructionScript
  (bind _outactors (Actor|GetAllActorsOfClass "/Game/BPActors/BP_Block.BP_Block_C"))
  (Variables|Default|SettotalNeeded (Utilities|Array|Length _outactors))
  (|CallParentFunction))