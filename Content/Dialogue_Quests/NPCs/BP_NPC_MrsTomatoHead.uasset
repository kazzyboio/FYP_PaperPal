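; Dialogue NPC Mrs. Tomato Head, whose dialogue state progresses in step with the Princess NPC's.
; Before dialogue starts, she looks up the Princess and advances from an even state to the next odd one when the Princess has reached it.
; After a states update, intermediate odd states step on to the next even, waiting state; the last state stays.
; A specific line in one state swaps her mesh to a crowned vertex-animation variant.
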(event EventDialogueEvent
  ;[1 1 1] Change Hat
  (if (and (== 3 (Variables|Default|GetstateIndex)) (== 6 (Variables|Default|GetdialogueIndex)))
    (Components|StaticMesh|SetStaticMesh (Variables|Default|GetStaticMesh) "/Game/Assets/NPCs/LadyTomatoWoman/Crowned/Crowned_MrsTomatoWoman_VertexAnimation_Mesh.Crowned_MrsTomatoWoman_VertexAnimation_Mesh"))
  (|CallParentFunction))

(event EventPreStartDialogue
  ;[1 1 1] Check for Princess Updates
  (bind _returnvalue (Actor|GetActorOfClass "/Game/Dialogue_Quests/NPCs/BP_NPC_Princess.BP_NPC_Princess_C"))
  (if (and (== (Variables|/Game/Dialogue_Quests/NPCs/BP_NPC.BP_NPC_C|GetstateIndex _returnvalue) 1) (== (Variables|Default|GetstateIndex) 0))
    (Variables|Default|SetstateIndex 1)
    (elif (and (== (Variables|/Game/Dialogue_Quests/NPCs/BP_NPC.BP_NPC_C|GetstateIndex _returnvalue) 3) (== (Variables|Default|GetstateIndex) 2))
      (Variables|Default|SetstateIndex 3)
      (elif (and (== (Variables|/Game/Dialogue_Quests/NPCs/BP_NPC.BP_NPC_C|GetstateIndex _returnvalue) 5) (== (Variables|Default|GetstateIndex) 4))
        (Variables|Default|SetstateIndex 5))))
  (|CallParentFunction))

(event EventPostStatesUpdate
  ;[1 1 1] Post States Update
  (if (== (Variables|Default|GetstateIndex) 1)
    (Variables|Default|SetstateIndex 2)
    (elif (== (Variables|Default|GetstateIndex) 3)
      (Variables|Default|SetstateIndex 4))))

(fn ConstructionScript
  (|CallParentFunction))