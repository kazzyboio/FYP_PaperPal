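; Mr. Tomato Head NPC, a dialogue character child Blueprint serving either a castle quest or a key quest, chosen by RowName.
; StateIndex tracks progress through overridden parent dialogue events.
; The castle variant reacts to the gate opening, then fades, moves to a target point and shows an input-specific tutorial.
; The key variant tracks acceptance and key pickup, swapping its mesh behind a mid-dialogue fade with sound.
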(event Custom|Gate%20Opened
  ;[1 1 1] Gate Event
  (if (== (Variables|Default|GetstateIndex) 1)
    (Variables|Default|SetstateIndex 2)
    (Utilities|FlowControl|Delay 0.5)
    (Transformation|SetActorRotation "0,195.000000, 0")
    (Transformation|SetRelativeLocation (Variables|Default|GetPlayerTeleport) "0,220.000000,25.000000" false false)
    (Variables|Default|SetpastGate true)
    (CallFunction|ActivateDialogue)))

(event EventPreStartDialogue
  ;[1 1 1] Check for Key
  (if (Variables|Default|GetkeyGot)
    (if (!= (Variables|Default|GetstateIndex) 0)
      (Variables|Default|SetstateIndex 3)
      (else
        (Variables|Default|SetstateIndex 2))))
  (|CallParentFunction))

(event EventReactivateMovement
  ;[1 1 1] Reactivate Movement
  (if (== (Variables|Default|GetRow%20Name) "Mr_Tomato_Castle")
    (if (!= (Variables|Default|GetstateIndex) 2)
      (|CallParentFunction :!label _label))
    (else
      (goto _label))))

(event EventDialogueEvent
  (bind _dialogueui (Variables|Default|GetdialogueUI))
  ;[1 1 1] Fade Event (Key Quest)
  (if (== (Variables|Default|GetRow%20Name) "Mr_Tomato_Castle")
    _
    (elif (or (and (== (Variables|Default|GetstateIndex) 2) (== (Variables|Default|GetdialogueIndex) 2)) (and (== (Variables|Default|GetstateIndex) 3) (== (Variables|Default|GetdialogueIndex) 8)))
      (Variables|Default|SetdialoguePlaying false)
      (Default|DespawnWidget (Variables|Default|GetdialogueUI))
      (CallFunction|StartFade)
      (Utilities|FlowControl|Delay 0.6)
      (Audio|PlaySound2D "/Game/Assets/SFX/SFX_Chest.SFX_Chest" 1.0 1.0 0.0 0 0)
      (Components|StaticMesh|SetStaticMesh (Variables|Default|GetStaticMesh) "/Game/Assets/NPCs/SirTomatoMan/Intact/MrTomatoMan_VertexAnimation.MrTomatoMan_VertexAnimation")
      (Utilities|FlowControl|Delay 1.8)
      (Variables|Default|SetdialoguePlaying true)
      (UserInterface|Viewport|AddtoViewport _dialogueui 0)
      (Default|SpawnWidget _dialogueui)
      (Audio|PlaySound2D (Variables|Default|GetdialogueSound) 1.0 1.0 0.0 0 0)))
  (|CallParentFunction))

(event EventPostStatesUpdate
  ;[1 1 1] Post States Update (Castle Quest)
  (if (== (Variables|Default|GetRow%20Name) "Mr_Tomato_Castle")
    (if (!= (Variables|Default|GetstateIndex) 2)
      (if (== (Variables|Default|GetstateIndex) 0)
        (Variables|Default|SetstateIndex 1)
        (Components|Sphere|SetSphereRadius (Variables|Default|GetSphereCollision) 2e+02 true))
      (else
        ;[1 1 1] Teleport
        (Variables|Default|SetdialogueStart true)
        (CallFunction|StartFade)
        (Utilities|FlowControl|Delay (Variables|Default|GetfadeDelay))
        (Transformation|SetActorRelativeLocation (Transformation|GetWorldLocation (Variables|/Script/Engine.Actor|GetRootComponent (Variables|Default|GettargetPoint))))
        (Transformation|SetActorRotation "0.000000,295.000000,0.000000")
        (Utilities|FlowControl|Delay (Variables|Default|GetfadeDelay))
        (|CallParentFunction)
        (Variables|Default|SetstateIndex 3)
        (Variables|Default|SetdialogueStart false)
        ;[1 1 1] Tutorial Pop Up
        (bind _asbp_player (Utilities|Casting|CastToBP_Player (Game|GetPlayerCharacter 0)))
        (switch Utilities|FlowControl|Switch|SwitchonInputDevice (Variables|/Game/PlayerCharacter/BP_Player.BP_Player_C|GetCurrentInputDevice _asbp_player)
          (:NewEnumerator0
            (bind _returnvalue (UserInterface|CreateWidget "/Game/Assets/UI/WB/WB_Tutorial.WB_Tutorial_C"))
            (UserInterface|Viewport|AddtoViewport _returnvalue 0)
            (Default|RollTutorialAniKBM _returnvalue))
          (:NewEnumerator1
            (bind _returnvalue_2 (UserInterface|CreateWidget "/Game/Assets/UI/WB/WB_Tutorial.WB_Tutorial_C"))
            (UserInterface|Viewport|AddtoViewport _returnvalue_2 0)
            (Default|RollTutorialAniPad _returnvalue_2)))))
    (else
      ;[1 1 1] Post States Update (Key Quest)
      (if (== (Variables|Default|GetstateIndex) 0)
        (Variables|Default|SetstateIndex 1)
        (Variables|Default|SetkeyQuestAccepted true)
        (elif (or (== (Variables|Default|GetstateIndex) 2) (== (Variables|Default|GetstateIndex) 3))
          (Variables|Default|SetstateIndex 4))))))

(fn ConstructionScript
  (|CallParentFunction))