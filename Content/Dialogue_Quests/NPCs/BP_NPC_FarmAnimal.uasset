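; Farm animal NPC that the player talks to as part of the Farmer's quest.
; Before dialogue starts, it moves to its quest state if BP_NPC_Farmer's quest is accepted.
; When that state completes, it updates the Farmer's quest, fades, teleports to a target point after a delay, resizes its interaction sphere and enters its final state.
; The parent's movement reactivation is held back until the relocation finishes.
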(event EventPreStartDialogue
  ;[1 1 1] Check for Farmer Quest Acceptance
  (bind _returnvalue (Actor|GetActorOfClass "/Game/Dialogue_Quests/NPCs/BP_NPC_Farmer.BP_NPC_Farmer_C"))
  (if (and (Variables|/Game/Dialogue_Quests/NPCs/BP_NPC_Farmer.BP_NPC_Farmer_C|GetquestAccepted _returnvalue) (== (Variables|Default|GetstateIndex) 0))
    (Variables|Default|SetstateIndex 1))
  (|CallParentFunction))

(event EventReactivateMovement
  ;[1 1 1] Lock Movement for Fade
  (if (!= (Variables|Default|GetstateIndex) 1)
    (|CallParentFunction)))

(event EventPostStatesUpdate
  ;[1 1 1] Update Farmer Quest
  (if (== (Variables|Default|GetstateIndex) 1)
    (bind _returnvalue (Actor|GetActorOfClass "/Game/Dialogue_Quests/NPCs/BP_NPC_Farmer.BP_NPC_Farmer_C"))
    (Default|QuestUpdate _returnvalue)
    ;[1 1 1] Fade Event
    (Variables|Default|SetdialogueStart true)
    (Default|DespawnWidget (Variables|Default|GetdialogueUI))
    (CallFunction|StartFade)
    (Utilities|FlowControl|Delay (Variables|Default|GetfadeDelay))
    (Transformation|SetActorLocation (Transformation|GetWorldLocation (Variables|/Script/Engine.Actor|GetRootComponent (Variables|Default|GettargetPoint))) false false)
    (Components|Sphere|SetSphereRadius (Variables|Default|GetSphereCollision) 1.5e+02 true)
    (Variables|Default|SetstateIndex 2)
    (Variables|Default|SetdialogueStart false)
    (|CallParentFunction)))

(fn ConstructionScript
  (|CallParentFunction))