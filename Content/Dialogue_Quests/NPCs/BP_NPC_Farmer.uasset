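; BP_NPC_Farmer is a quest-giving NPC whose dialogue state index follows a collection quest.
; Before dialogue, it switches to an alternate opening state if Mr Tomato Head's key quest is accepted; finishing either opening accepts the farmer's quest.
; QuestUpdate counts collected items and, at the target, spawns a data-table-driven self-dialogue actor at the player.
; Completing the turn-in dialogue adds a guest to the Monkey Pirate and updates the player's journal.
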(event Custom|Quest%20Update
  (bind _returnvalue (Game|GetPlayerCharacter 0))
  (bind _rootcomponent (Variables|/Script/Engine.Actor|GetRootComponent _returnvalue))
  ;[1 1 1] Quest Update
  (Variables|Default|SetstateIndex 3)
  (bind _result (Math|Integer|IncrementInt (Variables|Default|GettotalCollected))
    (:%20%20
      (if (== _result (Variables|Default|GettotalNeeded))
        (Variables|Default|SetstateIndex 4)
        (bind _output_get (Variables|Default|SetSpawn%20Transform (Math|Transform|MakeTransform (Transformation|GetWorldLocation _rootcomponent) (Transformation|GetWorldRotation _rootcomponent) "1.000000,1.000000,1.000000")))
        (bind _returnvalue_2 (Game|SpawnActorfromClass "/Game/Dialogue_Quests/NPCs/BP_NPC_SelfDialogue.BP_NPC_SelfDialogue_C" _output_get "Undefined" 0 0))
        (bind _output_get_2 (Variables|/Game/Dialogue_Quests/NPCs/BP_NPC.BP_NPC_C|SetRow%20Name _returnvalue_2 "Self_Dialogue_Farmer"))
        (bind _returnvalue_3 (Utilities|GetDataTableRow "/Game/Dialogue_Quests/DataTables/DT_NPCScripts.DT_NPCScripts" _output_get_2)
          (:then
            (Variables|/Game/Dialogue_Quests/NPCs/BP_NPC.BP_NPC_C|SetDialogue%20States _returnvalue_2 (.dialogueStates (Utilities|Struct|BreakStruct_NPCInfo _returnvalue_3)))
            (Variables|/Game/Dialogue_Quests/NPCs/BP_NPC.BP_NPC_C|SetType%20Speed _returnvalue_2 (.typeSpeed (Utilities|Struct|BreakStruct_NPCInfo _returnvalue_3)))))))))

(event EventPreStartDialogue
  ;[1 1 1] Mr Tomato Quest Check
  (bind _returnvalue (Actor|GetActorOfClass "/Game/Dialogue_Quests/NPCs/BP_NPC_MrTomatoHead.BP_NPC_MrTomatoHead_C"))
  (if (and (Variables|/Game/Dialogue_Quests/NPCs/BP_NPC_MrTomatoHead.BP_NPC_MrTomatoHead_C|GetkeyQuestAccepted _returnvalue) (== (Variables|Default|GetstateIndex) 0))
    (Variables|Default|SetstateIndex 1))
  (|CallParentFunction))

(event EventPostStatesUpdate
  ;[1 1 1] First Encounter Updates
  (if (or (== (Variables|Default|GetstateIndex) 0) (== (Variables|Default|GetstateIndex) 1))
    (Variables|Default|SetstateIndex 2)
    (Variables|Default|SetquestAccepted true)
    (elif (== (Variables|Default|GetstateIndex) 4)
      (Variables|Default|SetstateIndex 5)
      (bind _returnvalue (Actor|GetActorOfClass "/Game/Dialogue_Quests/NPCs/BP_NPC_MonkeyPirate.BP_NPC_MonkeyPirate_C"))
      (Default|AddGuest _returnvalue)
      (bind _returnvalue_2 (Actor|GetActorOfClass "/Game/PlayerCharacter/BP_Player.BP_Player_C"))
      (Default|FarmerDone (Variables|/Game/PlayerCharacter/BP_Player.BP_Player_C|GetJournalUI _returnvalue_2)))))

(fn ConstructionScript
  (|CallParentFunction))