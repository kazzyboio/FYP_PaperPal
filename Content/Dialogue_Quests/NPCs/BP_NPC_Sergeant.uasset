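; Sergeant quest NPC who has the player collect soldiers, then counts toward the Monkey Pirate's party guests.
; Once the party quest is accepted, Tick restages the scene once, revealing hidden soldiers and balloons.
; StateIndex drives progress from quest updates through a faded soldier regroup at target points to guest and journal updates.
; Overrides parent dialogue hooks, including a mid-dialogue blended camera pan that temporarily hides the dialogue UI.
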(event Custom|Quest%20Update
  ;[1 1 1] Quest Update
  (bind _result (Math|Integer|IncrementInt (Variables|Default|GettotalCollected))
    (:%20%20
      (if (== _result (Variables|Default|GettotalNeeded))
        (if (!= (Variables|Default|GetstateIndex) 0)
          (Variables|Default|SetstateIndex 3)
          (else
            (Variables|Default|SetstateIndex 4)))
        (bind _outactors (Actor|GetAllActorsOfClass "/Game/Dialogue_Quests/NPCs/BP_NPC_Soldier.BP_NPC_Soldier_C"))
        (Variables|Default|SetsoldierList _outactors)))))

(event Custom|Regroup%20Soldiers
  ;[1 1 1] Teleport Soldiers to Sergeant
  (Variables|Default|SetdialoguePlaying false)
  (Default|DespawnWidget (Variables|Default|GetdialogueUI))
  (CallFunction|StartFade)
  (Utilities|FlowControl|Delay (Variables|Default|GetfadeDelay))
  (for (_array_element _array_index) (Variables|Default|GetsoldierList)
    (Transformation|SetActorLocation _array_element (Transformation|GetWorldLocation (Variables|/Script/Engine.Actor|GetRootComponent (Utilities|Array|Get(acopy) (Variables|Default|GettargetPointsList) _array_index))) false false)
    (Transformation|SetActorRotation _array_element (Variables|Default|GetSoldier%20New%20Rotation))
    (Variables|/Game/Dialogue_Quests/NPCs/BP_NPC.BP_NPC_C|SetstateIndex _array_element 3)
    (Components|Sphere|SetSphereRadius (Variables|/Game/Dialogue_Quests/NPCs/BP_NPC.BP_NPC_C|GetSphereCollision _array_element) 125.0 true))
  (if (== (Variables|Default|GetstateIndex) 4)
    (Variables|Default|SetstateIndex 6)
    (|CallParentFunction)))

(event EventDialogueEvent
  (bind _dialogueui (Variables|Default|GetdialogueUI))
  (bind _blendtime (Variables|Default|GetblendTime))
  (bind _blendtime_2 (Variables|Default|GetblendTime))
  ;[1 1 1] Camera Pan
  (if (and (== 1 (Variables|Default|GetstateIndex)) (== 2 (Variables|Default|GetdialogueIndex)))
    (Variables|Default|SetdialoguePlaying false)
    (Default|DespawnWidget (Variables|Default|GetdialogueUI))
    (Game|Player|SetViewTargetwithBlend (Game|GetPlayerController 0) (Variables|Default|GetcameraActor) _blendtime_2 "VTBlend_Cubic" 0.0 false)
    (Utilities|FlowControl|Delay (+ _blendtime_2 (Variables|Default|GetcameraStayTime)))
    (Game|Player|SetViewTargetwithBlend (Game|GetPlayerController 0) (Components|GetOwner (Variables|Default|GetCamera)) _blendtime "VTBlend_Cubic" 0.0 false)
    (Utilities|FlowControl|Delay _blendtime)
    (Variables|Default|SetdialoguePlaying true)
    (UserInterface|Viewport|AddtoViewport _dialogueui 0)
    (Default|SpawnWidget _dialogueui)
    (Audio|PlaySound2D (Variables|Default|GetdialogueSound) 1.0 1.0 0.0 0 0))
  (|CallParentFunction))

(event EventReactivateMovement
  ;[1 1 1] Lock Movement for Fade
  (if (or (!= (Variables|Default|GetstateIndex) 3) (!= (Variables|Default|GetstateIndex) 4))
    (|CallParentFunction)))

(event EventPreStartDialogue
  ;[1 1 1] Monkey Pirate Quest Check
  (bind _returnvalue (Actor|GetActorOfClass "/Game/Dialogue_Quests/NPCs/BP_NPC_MonkeyPirate.BP_NPC_MonkeyPirate_C"))
  (if (and (Variables|/Game/Dialogue_Quests/NPCs/BP_NPC_MonkeyPirate.BP_NPC_MonkeyPirate_C|GetpartyQuestAccepted _returnvalue) (== (Variables|Default|GetstateIndex) 0))
    (Variables|Default|SetstateIndex 1))
  (|CallParentFunction))

(event EventPostStatesUpdate
  ;[1 1 1] First Encounter Updates
  (if (== (Variables|Default|GetstateIndex) 1)
    (Variables|Default|SetstateIndex 2)
    (elif (or (== (Variables|Default|GetstateIndex) 3) (== (Variables|Default|GetstateIndex) 4))
      (Variables|Default|SetstateIndex 5)
      (CallFunction|RegroupSoldiers)
      (elif (or (== (Variables|Default|GetstateIndex) 5) (== (Variables|Default|GetstateIndex) 6))
        (Variables|Default|SetstateIndex 7)
        (bind _returnvalue (Actor|GetActorOfClass "/Game/Dialogue_Quests/NPCs/BP_NPC_MonkeyPirate.BP_NPC_MonkeyPirate_C"))
        (Default|AddGuest _returnvalue)
        (bind _returnvalue_2 (Actor|GetActorOfClass "/Game/PlayerCharacter/BP_Player.BP_Player_C"))
        (Default|SoldierDone (Variables|/Game/PlayerCharacter/BP_Player.BP_Player_C|GetJournalUI _returnvalue_2))))))

(event EventTick
  (params (DeltaSeconds :type Float%20%28single-precision%29))
  (bind _extrameshes (Variables|Default|GetextraMeshes))
  ;[1 1 1] Post Monkey Pirate Changes
  (bind _returnvalue (Actor|GetActorOfClass "/Game/Dialogue_Quests/NPCs/BP_NPC_MonkeyPirate.BP_NPC_MonkeyPirate_C"))
  (if (and (Variables|Default|GetsoldiersTeleport) (Variables|/Game/Dialogue_Quests/NPCs/BP_NPC_MonkeyPirate.BP_NPC_MonkeyPirate_C|GetpartyQuestAccepted _returnvalue))
    (bind _output_get (Variables|Default|SetplayerLocation "0,160.000000, 0"))
    (Transformation|SetRelativeLocation (Variables|Default|GetPlayerTeleport) _output_get false false)
    (Transformation|SetRelativeLocationAndRotation (Variables|Default|GetCamera) "-192.000000,85.000000,60.000000" "-19.920664,0.000000,0.000000" false false)
    (Variables|Default|SetplayerRotationOffset -9e+01)
    (for _array_element _extrameshes
      (Actor|DestroyActor _array_element))
    (Utilities|Array|Clear _extrameshes)
    (bind _outactors (Actor|GetAllActorsOfClass "/Game/Dialogue_Quests/NPCs/BP_NPC_Soldier.BP_NPC_Soldier_C"))
    (bind _output_get_2 (Variables|Default|SetsoldierList _outactors))
    (for _array_element_2 _output_get_2
      (Rendering|SetActorHiddenInGame _array_element_2 false))
    (bind _outactors_2 (Actor|GetAllActorsOfClass "/Game/BPActors/BP_Balloon.BP_Balloon_C"))
    (for _array_element_3 _outactors_2
      (Rendering|SetActorHiddenInGame _array_element_3 false)
      (Collision|SetCollisionProfileName (Variables|/Game/BPActors/BP_Balloon.BP_Balloon_C|GetSphere _array_element_3) "BlockAllDynamic" true :!class /Script/Engine.PrimitiveComponent))
    (Variables|Default|SetsoldiersTeleport false)))

(fn ConstructionScript
  (|CallParentFunction))