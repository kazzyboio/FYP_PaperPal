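; Snail NPC dialogue Blueprint for the Monkey Pirate's party quest, with slow-talker handling through a per-speaker type speed.
; Before dialogue, it moves from state 0 to 1 if the pirate's party quest is accepted.
; After the state update, state 1 becomes 2, adding a guest to the pirate and marking the snail done in the player's journal.
; TypeText and SkipText overrides give snail lines their own speed and allow skipping only on "PP" lines.
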(event EventSkipText
  ;[1 1 1] Prevent Skipping on Snail
  (if (== (Variables|Default|GetcurrentName) "PP")
    (|CallParentFunction)))

(event EventPreStartDialogue
  ;[1 1 1] Check for Post Monkey Pirate
  (bind _returnvalue (Actor|GetActorOfClass "/Game/Dialogue_Quests/NPCs/BP_NPC_MonkeyPirate.BP_NPC_MonkeyPirate_C"))
  (if (and (Variables|/Game/Dialogue_Quests/NPCs/BP_NPC_MonkeyPirate.BP_NPC_MonkeyPirate_C|GetpartyQuestAccepted _returnvalue) (== (Variables|Default|GetstateIndex) 0))
    (Variables|Default|SetstateIndex 1))
  (|CallParentFunction))

(event EventPostStatesUpdate
  ;[1 1 1] Quest Accept + Complete
  (if (== (Variables|Default|GetstateIndex) 1)
    (Variables|Default|SetstateIndex 2)
    (bind _returnvalue (Actor|GetActorOfClass "/Game/Dialogue_Quests/NPCs/BP_NPC_MonkeyPirate.BP_NPC_MonkeyPirate_C"))
    (Default|AddGuest _returnvalue)
    (bind _returnvalue_2 (Actor|GetActorOfClass "/Game/PlayerCharacter/BP_Player.BP_Player_C"))
    (Default|Snaildone (Variables|/Game/PlayerCharacter/BP_Player.BP_Player_C|GetJournalUI _returnvalue_2))))

(event EventTypeText
  ;[1 1 1] Change Text Speeds
  (if (== (Variables|Default|GetcurrentName) "PP")
    (Variables|Default|SetType%20Speed 0.02)
    (|CallParentFunction :!label _label)
    (elif (or (== (Variables|Default|GetcurrentName) "SN") (== (Variables|Default|GetcurrentName) "?"))
      (Variables|Default|SetType%20Speed (Variables|Default|GetsnailTypeSpeed))
      (goto _label))))

(fn ConstructionScript
  (|CallParentFunction))