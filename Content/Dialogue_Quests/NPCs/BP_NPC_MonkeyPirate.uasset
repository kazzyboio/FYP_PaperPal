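; Monkey pirate quest NPC that runs the sword-collection quest and the party guest quest that follows it, through to the alpha end screen.
; Inserted sword counts drive sword animations and a dialogue StateIndex, which triggers quest accepts, camera pan and guest-list popup.
; The final sword swaps static characters for talkable NPCs with data-table dialogue and relocates the guards.
; Reaching the guest total spawns a self-dialogue NPC and sets the ending state.
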(event Custom|Add%20Guest
  (bind _returnvalue (Game|GetPlayerCharacter 0))
  (bind _rootcomponent (Variables|/Script/Engine.Actor|GetRootComponent _returnvalue))
  ;[1 1 1] Add Guest
  (bind _result (Math|Integer|IncrementInt (Variables|Default|GettotalInvited))
    (:%20%20
      (if (== _result (Variables|Default|GettotalGuests))
        (Variables|Default|SetstateIndex 8)
        (bind _output_get (Variables|Default|SetselfDialogueTransform (Math|Transform|MakeTransform (Transformation|GetWorldLocation _rootcomponent) (Transformation|GetWorldRotation _rootcomponent) "1.000000,1.000000,1.000000")))
        (bind _returnvalue_2 (Game|SpawnActorfromClass "/Game/Dialogue_Quests/NPCs/BP_NPC_SelfDialogue.BP_NPC_SelfDialogue_C" _output_get "Undefined" 0 0))
        (bind _output_get_2 (Variables|/Game/Dialogue_Quests/NPCs/BP_NPC.BP_NPC_C|SetRow%20Name _returnvalue_2 "Self_Dialogue_Guests"))
        (bind _returnvalue_3 (Utilities|GetDataTableRow "/Game/Dialogue_Quests/DataTables/DT_NPCScripts.DT_NPCScripts" _output_get_2)
          (:then
            (Variables|/Game/Dialogue_Quests/NPCs/BP_NPC.BP_NPC_C|SetDialogue%20States _returnvalue_2 (.dialogueStates (Utilities|Struct|BreakStruct_NPCInfo _returnvalue_3)))
            (Variables|/Game/Dialogue_Quests/NPCs/BP_NPC.BP_NPC_C|SetType%20Speed _returnvalue_2 (.typeSpeed (Utilities|Struct|BreakStruct_NPCInfo _returnvalue_3)))))))))

(event Custom|Post%20Launch%20Spawns
  ;[1 1 1] Mr Tomato + Farmer Spawn
  (bind _returnvalue (Actor|GetActorOfClass "/Game/Dialogue_Quests/Static_MrTomato.Static_MrTomato_C"))
  (Actor|DestroyActor _returnvalue)
  (bind _output_get (Variables|Default|SetmrTomatoTransform (Math|Transform|MakeTransform (+ (Transformation|GetWorldLocation (Variables|/Script/Engine.Actor|GetRootComponent (Variables|Default|GetmrTomatoSpawnPoint))) "0,0,52.000000") (Variables|Default|GetmrTomatoSpawnRotation) "1.000000,1.000000,1.000000")))
  (bind _returnvalue_2 (Game|SpawnActorfromClass "/Game/Dialogue_Quests/NPCs/BP_NPC_MrTomatoHead.BP_NPC_MrTomatoHead_C" _output_get "Undefined" 0 0))
  (Components|StaticMesh|SetStaticMesh (Variables|/Game/Dialogue_Quests/NPCs/BP_NPC.BP_NPC_C|GetStaticMesh _returnvalue_2) "/Game/Assets/NPCs/SirTomatoMan/Mutilated/MrTomatoManMutilated_VertexAnimation.MrTomatoManMutilated_VertexAnimation")
  (bind _output_get_2 (Variables|/Game/Dialogue_Quests/NPCs/BP_NPC.BP_NPC_C|SetRow%20Name _returnvalue_2 "Mr_Tomato_Key"))
  (bind _returnvalue_3 (Utilities|GetDataTableRow "/Game/Dialogue_Quests/DataTables/DT_NPCScripts.DT_NPCScripts" _output_get_2)
    (:then
      (Variables|/Game/Dialogue_Quests/NPCs/BP_NPC.BP_NPC_C|SetDialogue%20States _returnvalue_2 (.dialogueStates (Utilities|Struct|BreakStruct_NPCInfo _returnvalue_3)))
      (Variables|/Game/Dialogue_Quests/NPCs/BP_NPC.BP_NPC_C|SetType%20Speed _returnvalue_2 (.typeSpeed (Utilities|Struct|BreakStruct_NPCInfo _returnvalue_3)))
      (bind _returnvalue_4 (Actor|GetActorOfClass "/Game/Dialogue_Quests/Static_Guard.Static_Guard_C"))
      (Actor|DestroyActor _returnvalue_4)
      (bind _output_get_3 (Variables|Default|SetfarmerTransform (Math|Transform|MakeTransform (+ (Transformation|GetWorldLocation (Variables|/Script/Engine.Actor|GetRootComponent (Variables|Default|GetfarmerSpawnPoint))) "0,0,52.000000") (Variables|Default|GetfarmerSpawnRotation) "1.000000,1.000000,1.000000")))
      (bind _returnvalue_5 (Game|SpawnActorfromClass "/Game/Dialogue_Quests/NPCs/BP_NPC_Farmer.BP_NPC_Farmer_C" _output_get_3 "Undefined" 0 0))
      (bind _output_get_4 (Variables|/Game/Dialogue_Quests/NPCs/BP_NPC.BP_NPC_C|SetRow%20Name _returnvalue_5 "Farmer"))
      (bind _returnvalue_6 (Utilities|GetDataTableRow "/Game/Dialogue_Quests/DataTables/DT_NPCScripts.DT_NPCScripts" _output_get_4)
        (:then
          (Variables|/Game/Dialogue_Quests/NPCs/BP_NPC.BP_NPC_C|SetDialogue%20States _returnvalue_5 (.dialogueStates (Utilities|Struct|BreakStruct_NPCInfo _returnvalue_6)))
          (Variables|/Game/Dialogue_Quests/NPCs/BP_NPC.BP_NPC_C|SetType%20Speed _returnvalue_5 (.typeSpeed (Utilities|Struct|BreakStruct_NPCInfo _returnvalue_6)))
          ;[1 1 1] Mrs Tomato + Princess Spawn
          (bind _returnvalue_7 (Actor|GetActorOfClass "/Game/Dialogue_Quests/Static_Princess.Static_Princess_C"))
          (Actor|DestroyActor _returnvalue_7)
          (bind _returnvalue_8 (Actor|GetActorOfClass "/Game/Dialogue_Quests/Static_MrsTomato.Static_MrsTomato_C"))
          (Actor|DestroyActor _returnvalue_8)
          (bind _output_get_5 (Variables|Default|SetprincessSpawnTransform (Math|Transform|MakeTransform (+ (Transformation|GetWorldLocation (Variables|/Script/Engine.Actor|GetRootComponent (Variables|Default|GetprincessSpawnPoint))) "0,0,52.000000") (Variables|Default|GetprincessSpawnRotation) "1.000000,1.000000,1.000000")))
          (bind _returnvalue_9 (Game|SpawnActorfromClass "/Game/Dialogue_Quests/NPCs/BP_NPC_Princess.BP_NPC_Princess_C" _output_get_5 "Undefined" 0 0))
          (bind _output_get_6 (Variables|/Game/Dialogue_Quests/NPCs/BP_NPC.BP_NPC_C|SetRow%20Name _returnvalue_9 "Princess_Party"))
          (bind _returnvalue_10 (Utilities|GetDataTableRow "/Game/Dialogue_Quests/DataTables/DT_NPCScripts.DT_NPCScripts" _output_get_6)
            (:then
              (Variables|/Game/Dialogue_Quests/NPCs/BP_NPC.BP_NPC_C|SetDialogue%20States _returnvalue_9 (.dialogueStates (Utilities|Struct|BreakStruct_NPCInfo _returnvalue_10)))
              (Variables|/Game/Dialogue_Quests/NPCs/BP_NPC.BP_NPC_C|SetType%20Speed _returnvalue_9 (.typeSpeed (Utilities|Struct|BreakStruct_NPCInfo _returnvalue_10)))
              (Variables|/Game/Dialogue_Quests/NPCs/BP_NPC.BP_NPC_C|SetplayerLocation _returnvalue_9 "0,320.000000,-55.000000")
              (Variables|/Game/Dialogue_Quests/NPCs/BP_NPC.BP_NPC_C|SetcameraTransform _returnvalue_9 (Math|Transform|MakeTransform "-342.000000,576.000000,153.000000" "-19.920664,-45.319103,1.816933" "1.000000,1.000000,1.000000"))
              (Components|Sphere|SetSphereRadius (Variables|/Game/Dialogue_Quests/NPCs/BP_NPC.BP_NPC_C|GetSphereCollision _returnvalue_9) 3.5e+02 true)
              (bind _output_get_7 (Variables|Default|SetmrsTomatoTransform (Math|Transform|MakeTransform (+ (Transformation|GetWorldLocation (Variables|/Script/Engine.Actor|GetRootComponent (Variables|Default|GetmrsTomatoSpawnPoint))) "0,0,52.000000") (Variables|Default|GetmrsTomatoSpawnRotation) "1.000000,1.000000,1.000000")))
              (bind _returnvalue_11 (Game|SpawnActorfromClass "/Game/Dialogue_Quests/NPCs/BP_NPC_MrsTomatoHead.BP_NPC_MrsTomatoHead_C" _output_get_7 "Undefined" 0 0))
              (bind _output_get_8 (Variables|/Game/Dialogue_Quests/NPCs/BP_NPC.BP_NPC_C|SetRow%20Name _returnvalue_11 "Mrs_Tomato"))
              (bind _returnvalue_12 (Utilities|GetDataTableRow "/Game/Dialogue_Quests/DataTables/DT_NPCScripts.DT_NPCScripts" _output_get_8)
                (:then
                  (Variables|/Game/Dialogue_Quests/NPCs/BP_NPC.BP_NPC_C|SetDialogue%20States _returnvalue_11 (.dialogueStates (Utilities|Struct|BreakStruct_NPCInfo _returnvalue_12)))
                  (Variables|/Game/Dialogue_Quests/NPCs/BP_NPC.BP_NPC_C|SetType%20Speed _returnvalue_11 (.typeSpeed (Utilities|Struct|BreakStruct_NPCInfo _returnvalue_12)))
                  (bind _returnvalue_13 (Actor|GetActorOfClass "/Game/Dialogue_Quests/NPCs/BP_NPC_Guards.BP_NPC_Guards_C"))
                  (Transformation|SetActorLocationAndRotation _returnvalue_13 (+ (Transformation|GetWorldLocation (Variables|/Script/Engine.Actor|GetRootComponent (Variables|Default|GetguardNewPosition))) "0,0,52.000000") (Variables|Default|GetguardNewRotation))
                  (Variables|/Game/Dialogue_Quests/NPCs/BP_NPC.BP_NPC_C|SetplayerLocation _returnvalue_13 "0,160.000000,0.000000")
                  (Variables|/Game/Dialogue_Quests/NPCs/BP_NPC.BP_NPC_C|SetcameraTransform _returnvalue_13 (Math|Transform|MakeTransform "-192.000000,266.000000,163.000000" "-19.920664,-45.319103,1.816933" "1.000000,1.000000,1.000000"))
                  (Components|Sphere|SetSphereRadius (Variables|/Game/Dialogue_Quests/NPCs/BP_NPC.BP_NPC_C|GetSphereCollision _returnvalue_13) 175.0 true))))))))))

(event Custom|Play%20Animations
  ;[1 1 1] Animations
  (if (Variables|Default|GetfinalSword)
    (Variables|Default|SetfinalSword false)
    (Sequencer|Player|Play (Variables|/Script/LevelSequence.LevelSequenceActor|GetSequencePlayer (Variables|Default|GetlastSword)) :!class /Script/MovieScene.MovieSceneSequencePlayer)
    (Variables|Default|SetplayingAnimation true)
    (CallFunction|PostLaunchSpawns)
    (Utilities|FlowControl|Delay 4.5)
    (elif (== (Variables|Default|GettotalInserted) 3)
      (Sequencer|Player|Play (Variables|/Script/LevelSequence.LevelSequenceActor|GetSequencePlayer (Variables|Default|GetthirdSword)) :!class /Script/MovieScene.MovieSceneSequencePlayer)
      (if (Variables|Default|GetsecondPlayed)
        _
        (else
          (Sequencer|Player|Play (Variables|/Script/LevelSequence.LevelSequenceActor|GetSequencePlayer (Variables|Default|GetsecondSword)) :!class /Script/MovieScene.MovieSceneSequencePlayer :!label _label)
          (Variables|Default|SetsecondPlayed true)
          (if (Variables|Default|GetfirstPlayed)
            _
            (else
              (Sequencer|Player|Play (Variables|/Script/LevelSequence.LevelSequenceActor|GetSequencePlayer (Variables|Default|GetfirstSword)) :!class /Script/MovieScene.MovieSceneSequencePlayer :!label _label_2)
              (Variables|Default|SetfirstPlayed true)))))
      (Variables|Default|SetplayingAnimation true)
      (Utilities|FlowControl|Delay 1.5)
      (elif (== (Variables|Default|GettotalInserted) 2)
        (goto _label)
        (elif (== (Variables|Default|GettotalInserted) 1)
          (goto _label_2)
          (else
            _)))))
  (Variables|Default|SetplayingAnimation false)
  (CallFunction|StartDialogue))

(event Custom|Insert%20Sword
  ;[1 1 1] Insert Sword
  (if (not (Variables|Default|GetfinalSword))
    (Variables|Default|SettotalInserted (+ (Variables|Default|GettotalInserted) (Variables|Default|GettotalCollected)))
    (Variables|Default|SettotalCollected 0)
    (if (== (Variables|Default|GettotalInserted) (Variables|Default|GettotalNeeded))
      (Variables|Default|SetstateIndex 4)
      (else
        (Variables|Default|SetstateIndex 3)))
    (else
      (Variables|Default|SetstateIndex 6)))
  (CallFunction|PlayAnimations))

(event Custom|Add%20Sword
  ;[1 1 1] Add Sword
  (Math|Integer|IncrementInt (Variables|Default|GettotalCollected)))

(event EventCameraPan
  (bind _blendtime (Variables|Default|GetblendTime))
  (bind _stateindex (Variables|Default|GetstateIndex))
  ;[1 1 1] Camera Pan
  (if (or (== _stateindex 4) (== _stateindex 5))
    (Game|Player|SetViewTargetwithBlend (Game|GetPlayerController 0) (Variables|Default|GetcameraActor) _blendtime "VTBlend_Linear" 0.0 false)
    (Utilities|FlowControl|Delay (+ _blendtime (Variables|Default|GetcameraStayTime))))
  (|CallParentFunction))

(event EventReactivateMovement
  ;[1 1 1] Quest Update Changes
  (if (!= (Variables|Default|GetstateIndex) 6)
    (|CallParentFunction)))

(event EventPreStartDialogue
  ;[1 1 1] Insert Sword Check, Party Guests Count Check
  (if (not (Variables|Default|GetplayingAnimation))
    (if (Variables|Default|GetfinalSword)
      (CallFunction|InsertSword :!label _label)
      (elif (> (Variables|Default|GettotalCollected) 0)
        (goto _label)
        (else
          (|CallParentFunction))))))

(event EventPostStatesUpdate
  (bind _returnvalue (Game|GetPlayerController 0))
  ;[1 1 1] Quest Update Changes
  (if (Variables|Default|GetcastleQuestComplete)
    (if (== (Variables|Default|GetstateIndex) 1)
      (Variables|Default|SetstateIndex 2)
      (Variables|Default|SetquestAccepted true)
      (elif (and (== (Variables|Default|GetstateIndex) 3) (== (Variables|Default|GettotalCollected) 0))
        (Variables|Default|SetstateIndex 2)
        (elif (== (Variables|Default|GetstateIndex) 4)
          (Variables|Default|SetstateIndex 5)
          (bind _returnvalue_2 (Actor|GetActorOfClass "/Game/Dialogue_Quests/NPCs/BP_NPC_TrashPaper.BP_NPC_TrashPaper_C"))
          (Default|QuestAcceptChange _returnvalue_2)
          (elif (== (Variables|Default|GetstateIndex) 6)
            (Variables|Default|SetstateIndex 7)
            (Variables|Default|SetpartyQuestAccepted true)
            ;[1 1 1] Guest List Popup
            (Variables|Default|SetdialogueStart true)
            (bind _returnvalue_3 (Actor|GetActorOfClass "/Game/PlayerCharacter/BP_Player.BP_Player_C"))
            (Variables|/Game/PlayerCharacter/BP_Player.BP_Player_C|SetinDialogue _returnvalue_3 true)
            (bind _returnvalue_4 (UserInterface|CreateWidget "/Game/Assets/UI/WB/WB_GLPLACEHOLDER.WB_GLPLACEHOLDER_C" (Game|GetPlayerController 0)))
            (UserInterface|Viewport|AddtoViewport _returnvalue_4 0)
            (Default|SpawnAnimation _returnvalue_4)
            (Variables|Default|SetdialogueStart false)
            (elif (== (Variables|Default|GetstateIndex) 8)
              (bind _returnvalue_5 (UserInterface|CreateWidget "/Game/Assets/UI/WB/WB_EndScreenforAlpha.WB_EndScreenforAlpha_C" _returnvalue))
              (UserInterface|Viewport|AddtoViewport _returnvalue_5 0)
              (Input|SetInputModeUIOnly _returnvalue 0 "DoNotLock")
              (Variables|/Script/Engine.PlayerController|SetbShowMouseCursor _returnvalue true))))))))

(fn ConstructionScript
  (|CallParentFunction))