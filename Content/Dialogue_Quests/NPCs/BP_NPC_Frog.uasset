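; Frog quest NPC that changes its dialogue state once the Princess quest is accepted and reports back to her quest after talking.
; It overrides parent dialogue events to fade out and swap itself for a Static_Frog at a target point, registered with the MonkeyPirate.
; The first frog fades after dialogue and moves all frogs to state 2, so later ones fade mid-dialogue, then resume talking before being destroyed.
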(event EventDialogueEvent
  (bind _dialogueui (Variables|Default|GetdialogueUI))
  ;[1 1 1] Second Frog Fade (Dialogue After Fade)
  (if (and (== 2 (Variables|Default|GetstateIndex)) (== 1 (Variables|Default|GetdialogueIndex)))
    (Variables|Default|SetdialoguePlaying false)
    (Default|DespawnWidget (Variables|Default|GetdialogueUI))
    (CallFunction|StartFade)
    (Utilities|FlowControl|Delay (Variables|Default|GetfadeDelay))
    (Rendering|SetActorHiddenInGame true)
    (bind _returnvalue (Game|SpawnActorfromClass "/Game/Dialogue_Quests/StaticActors/Static_Frog.Static_Frog_C" (Variables|Default|GetSpawn%20Transform) "Undefined" 0 0))
    (Transformation|SetActorRelativeLocation _returnvalue (Transformation|GetWorldLocation (Variables|/Script/Engine.Actor|GetRootComponent (Variables|Default|GettargetPoint))))
    (bind _returnvalue_2 (Actor|GetActorOfClass "/Game/Dialogue_Quests/NPCs/BP_NPC_MonkeyPirate.BP_NPC_MonkeyPirate_C"))
    (Utilities|Array|Add (Variables|/Game/Dialogue_Quests/NPCs/BP_NPC_MonkeyPirate.BP_NPC_MonkeyPirate_C|GetstaticFrogs _returnvalue_2) _returnvalue)
    (Utilities|FlowControl|Delay (Variables|Default|GetfadeDelay))
    (Variables|Default|SetdialoguePlaying true)
    (UserInterface|Viewport|AddtoViewport _dialogueui 0)
    (Default|SpawnWidget _dialogueui)
    (Audio|PlaySound2D (Variables|Default|GettypeSoundA) 1.0 1.0 0.0 0 0))
  (|CallParentFunction))

(event EventReactivateMovement
  ;[1 1 1] Cancel Reactivate Movement
  (if (== (Variables|Default|GetstateIndex) 0)
    (|CallParentFunction)))

(event EventPreStartDialogue
  ;[1 1 1] Check Quest Accepted
  (bind _returnvalue (Actor|GetActorOfClass "/Game/Dialogue_Quests/NPCs/BP_NPC_Princess.BP_NPC_Princess_C"))
  (if (and (Variables|/Game/Dialogue_Quests/NPCs/BP_NPC_Princess.BP_NPC_Princess_C|GetquestAccepted _returnvalue) (== (Variables|Default|GetstateIndex) 0))
    (Variables|Default|SetstateIndex 1))
  (|CallParentFunction))

(event EventPostStatesUpdate
  ;[1 1 1] Update Princess Quest + First Frog Fade
  (if (!= 0 (Variables|Default|GetstateIndex))
    (bind _returnvalue (Actor|GetActorOfClass "/Game/Dialogue_Quests/NPCs/BP_NPC_Princess.BP_NPC_Princess_C"))
    (Default|QuestUpdate _returnvalue)
    (if (!= 2 (Variables|Default|GetstateIndex))
      (Variables|Default|SetdialogueStart true)
      (bind _returnvalue_2 (Actor|GetActorOfClass "/Game/PlayerCharacter/BP_Player.BP_Player_C"))
      (Variables|/Game/PlayerCharacter/BP_Player.BP_Player_C|SetinDialogue _returnvalue_2 true)
      (CallFunction|StartFade)
      (Utilities|FlowControl|Delay (Variables|Default|GetfadeDelay))
      (Rendering|SetActorHiddenInGame true)
      (bind _returnvalue_3 (Game|SpawnActorfromClass "/Game/Dialogue_Quests/StaticActors/Static_Frog.Static_Frog_C" (Variables|Default|GetSpawn%20Transform) "Undefined" 0 0))
      (Transformation|SetActorRelativeLocation _returnvalue_3 (Transformation|GetWorldLocation (Variables|/Script/Engine.Actor|GetRootComponent (Variables|Default|GettargetPoint))))
      (bind _returnvalue_4 (Actor|GetActorOfClass "/Game/Dialogue_Quests/NPCs/BP_NPC_MonkeyPirate.BP_NPC_MonkeyPirate_C"))
      (Utilities|Array|Add (Variables|/Game/Dialogue_Quests/NPCs/BP_NPC_MonkeyPirate.BP_NPC_MonkeyPirate_C|GetstaticFrogs _returnvalue_4) _returnvalue_3)
      (bind _outactors (Actor|GetAllActorsOfClass "BP_NPC_Frog_C"))
      (for _array_element _outactors
        (Variables|/Game/Dialogue_Quests/NPCs/BP_NPC.BP_NPC_C|SetstateIndex _array_element 2))
      (Utilities|FlowControl|Delay (Variables|Default|GetfadeDelay))
      (|CallParentFunction)
      (Variables|Default|SetdialogueStart false)
      (bind _returnvalue_5 (Actor|GetActorOfClass "/Game/PlayerCharacter/BP_Player.BP_Player_C"))
      (Variables|/Game/PlayerCharacter/BP_Player.BP_Player_C|SetinDialogue _returnvalue_5 false)
      (Actor|DestroyActor)
      (else
        (|CallParentFunction)
        (Actor|DestroyActor)))))

(fn ConstructionScript
  (|CallParentFunction))