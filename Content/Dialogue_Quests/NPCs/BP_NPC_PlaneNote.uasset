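; BP_NPC_PlaneNote is a dialogue/quest NPC Blueprint that shows the glide tutorial on its first encounter.
; On PostStatesUpdate it clears the FirstEncounter flag, then reads the current input device from BP_Player.
; It creates a WB_Tutorial widget, adds it to the viewport and plays the matching keyboard/mouse or gamepad glide animation.
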(event EventPostStatesUpdate
  ;[1 1 1] Tutorial Pop Up
  (if (Variables|Default|GetfirstEncounter)
    (Variables|Default|SetfirstEncounter false)
    (bind _asbp_player (Utilities|Casting|CastToBP_Player (Game|GetPlayerCharacter 0)))
    (switch Utilities|FlowControl|Switch|SwitchonInputDevice (Variables|/Game/PlayerCharacter/BP_Player.BP_Player_C|GetCurrentInputDevice _asbp_player)
      (:NewEnumerator0
        (bind _returnvalue (UserInterface|CreateWidget "/Game/Assets/UI/WB/WB_Tutorial.WB_Tutorial_C"))
        (UserInterface|Viewport|AddtoViewport _returnvalue 0)
        (Default|GlideTutorialAniKBM _returnvalue))
      (:NewEnumerator1
        (bind _returnvalue_2 (UserInterface|CreateWidget "/Game/Assets/UI/WB/WB_Tutorial.WB_Tutorial_C"))
        (UserInterface|Viewport|AddtoViewport _returnvalue_2 0)
        (Default|GlideTutorialAniPad _returnvalue_2)))))

(fn ConstructionScript
  (|CallParentFunction))