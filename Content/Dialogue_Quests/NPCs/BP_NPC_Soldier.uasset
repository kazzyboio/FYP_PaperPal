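; Soldier NPC for the Sergeant's rescue quest, extending a parent NPC's dialogue and state logic.
; Popping its balloon runs a per-soldier timeline on mesh height, then updates the Sergeant's quest and sets collision profiles after a delay.
; Before dialogue it checks whether the Sergeant's count is complete to enter state 2, which triggers regrouping after the state update and blocks the parent's movement reactivation.
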(event Custom|Pop%20Balloon
  ;[1 1 1] Pop Balloon
  (if (== (Variables|Default|GetRow%20Name) "Soldier_A")
    (bind _meshposition (Timeline|Timeline_1 Play)
      (:Update
        (Transformation|SetRelativeLocation (Variables|Default|GetStaticMesh) (Math|Vector|MakeVector 0.0 0.0 _meshposition) false false))
      (:Finished
        (bind _returnvalue (Actor|GetActorOfClass "/Game/Dialogue_Quests/NPCs/BP_NPC_Sergeant.BP_NPC_Sergeant_C" :!label _label))
        (Default|QuestUpdate _returnvalue)
        (Utilities|FlowControl|Delay 1.0)
        (Collision|SetCollisionProfileName (Variables|Default|GetSphereCollision) "OverlapAllDynamic" true :!class /Script/Engine.PrimitiveComponent)
        (Collision|SetCollisionProfileName (Variables|Default|GetCapsuleComponent) "BlockAllDynamic" true :!class /Script/Engine.PrimitiveComponent)))
    (elif (== (Variables|Default|GetRow%20Name) "Soldier_B")
      (bind _meshposition_2 (Timeline|Timeline_2 Play)
        (:Update
          (Transformation|SetRelativeLocation (Variables|Default|GetStaticMesh) (Math|Vector|MakeVector 0.0 0.0 _meshposition_2) false false))
        (:Finished
          (goto _label)))
      (else
        (bind _meshposition_3 (Timeline|Timeline_3 Play)
          (:Update
            (Transformation|SetRelativeLocation (Variables|Default|GetStaticMesh) (Math|Vector|MakeVector 0.0 0.0 _meshposition_3) false false))
          (:Finished
            (goto _label)))))))

(event EventPreStartDialogue
  ;[1 1 1] Check for All Soldiers Saved
  (bind _returnvalue (Actor|GetActorOfClass "/Game/Dialogue_Quests/NPCs/BP_NPC_Sergeant.BP_NPC_Sergeant_C"))
  (if (and (== (Variables|/Game/Dialogue_Quests/NPCs/BP_NPC_Sergeant.BP_NPC_Sergeant_C|GettotalCollected _returnvalue) (Variables|/Game/Dialogue_Quests/NPCs/BP_NPC_Sergeant.BP_NPC_Sergeant_C|GettotalNeeded _returnvalue)) (or (== (Variables|Default|GetstateIndex) 0) (== (Variables|Default|GetstateIndex) 1)))
    (Variables|Default|SetstateIndex 2))
  (|CallParentFunction))

(event EventReactivateMovement
  ;[1 1 1] Lock Movement for Fade
  (if (!= (Variables|Default|GetstateIndex) 2)
    (|CallParentFunction)))

(event EventPostStatesUpdate
  ;[1 1 1] First Encounter Updates
  (if (== (Variables|Default|GetstateIndex) 0)
    (Variables|Default|SetstateIndex 1)
    (elif (== (Variables|Default|GetstateIndex) 2)
      (bind _returnvalue (Actor|GetActorOfClass "/Game/Dialogue_Quests/NPCs/BP_NPC_Sergeant.BP_NPC_Sergeant_C"))
      (Default|RegroupSoldiers _returnvalue))))

(fn ConstructionScript
  (|CallParentFunction))