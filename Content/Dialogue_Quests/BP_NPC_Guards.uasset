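; BP_NPC_Guards is a quest NPC that auto-starts dialogue when the player enters its initial collision.
; PostStatesUpdate advances StateIndex, first starting the princess quest, repositioning its player teleport point and camera, and removing the initial collisions.
; From state 2, it completes the castle quest and sets the Monkey Pirate to auto-activate.
; Quest progress passes to other NPCs by finding their actors and setting state directly.
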(event OnComponentBeginOverlap(initialCollision)
  (params (OverlappedComponent :type Primitive%20Component%20Object%20Reference) (OtherActor :type Actor%20Object%20Reference) (OtherComp :type Primitive%20Component%20Object%20Reference) (OtherBodyIndex :type Integer) (bFromSweep :type Boolean) (SweepResult :type Hit%20Result%20Structure%20%28by%20ref%29))
  ;[1 1 1] Initial Auto Play Dialogue
  (Utilities|Casting|CastToBP_Player OtherActor)
  (CallFunction|EnterCollision))

(event EventPostStatesUpdate
  ;[1 1 1] Start Princess Quest
  (if (== (Variables|Default|GetstateIndex) 0)
    (Variables|Default|SetstateIndex 1)
    (bind _returnvalue (Actor|GetActorOfClass "/Game/Dialogue_Quests/BP_NPC_Princess.BP_NPC_Princess_C"))
    (Variables|/Game/Dialogue_Quests/BP_NPC_Princess.BP_NPC_Princess_C|SetquestAccepted _returnvalue true)
    (Variables|/Game/Dialogue_Quests/BP_NPC.BP_NPC_C|SetstateIndex _returnvalue 2)
    (Transformation|SetRelativeLocation (Variables|Default|GetPlayerTeleport) (Variables|Default|GetnewPlayerLocation) false false)
    (Transformation|SetRelativeTransform (Variables|Default|GetCamera) (Variables|Default|GetnewCameraTransform) false false)
    (bind _initialcollision (Variables|Default|GetinitialCollision)
      (:then
        (bind _initialstandcollision (Variables|Default|GetinitialStandCollision)
          (:then
            (Components|DestroyComponent _initialcollision)
            (Components|DestroyComponent _initialstandcollision))
          (:else)))
      (:else))
    (else
      ;[1 1 1] Complete Quest + Activate Monkey Pirate Quest
      (if (== (Variables|Default|GetstateIndex) 2)
        (Variables|Default|SetstateIndex 3)
        (bind _returnvalue_2 (Actor|GetActorOfClass "/Game/Dialogue_Quests/BP_NPC_MonkeyPirate.BP_NPC_MonkeyPirate_C"))
        (Variables|/Game/Dialogue_Quests/BP_NPC_MonkeyPirate.BP_NPC_MonkeyPirate_C|SetcastleQuestComplete _returnvalue_2 true)
        (Variables|/Game/Dialogue_Quests/BP_NPC.BP_NPC_C|SetstateIndex _returnvalue_2 1)
        (Variables|/Game/Dialogue_Quests/BP_NPC.BP_NPC_C|SetautoActivate _returnvalue_2 true)))))

(fn ConstructionScript
  (|CallParentFunction))