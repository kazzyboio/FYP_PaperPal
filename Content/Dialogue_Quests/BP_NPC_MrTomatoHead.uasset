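; Mr. TomatoHead dialogue NPC that steps through a StateIndex around a gate encounter and tutorial.
; Post-dialogue updates advance the first state; GateOpened then turns the NPC and starts the next dialogue.
; After that, it teleports to a TargetPoint behind a fade, restores player movement and jump-effect visibility, and shows the tutorial popup.
; ReactivateMovement restores movement and that effect in every state except the teleport one.
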(event Custom|Gate%20Opened
  ;[1 1 1] Gate Event
  (if (== (Variables|Default|GetstateIndex) 1)
    (Variables|Default|SetstateIndex 2)
    (Utilities|FlowControl|Delay 0.5)
    (Transformation|SetActorRotation "0,180.000000, 0")
    (Variables|Default|SetpastGate true)
    (CallFunction|ActivateDialogue)))

(event EventReactivateMovement
  ;[1 1 1] Reactivate Movement
  (if (not (== (Variables|Default|GetstateIndex) 2))
    (Components|Activation|Activate (Variables|/Script/Engine.Character|GetCharacterMovement (Game|GetPlayerCharacter 0)) false)
    (bind _returnvalue (Actor|GetActorOfClass "/Game/Characters/PlayerCharacter/BP_Player.BP_Player_C"))
    (Rendering|SetVisibility (Variables|/Game/Characters/PlayerCharacter/BP_Player.BP_Player_C|GetNS_Jump _returnvalue) true false)))

(event EventPostStatesUpdate
  ;[1 1 1] First Encounter Updates
  (if (not (== (Variables|Default|GetstateIndex) 2))
    (if (== (Variables|Default|GetstateIndex) 0)
      (Variables|Default|SetstateIndex 1))
    (else
      ;[1 1 1] Teleport
      (Variables|Default|SetdialogueStart true)
      (CallFunction|StartFade)
      (Utilities|FlowControl|Delay (Variables|Default|GetfadeDelay))
      (Transformation|SetActorRelativeLocation (Transformation|GetWorldLocation (Variables|/Script/Engine.Actor|GetRootComponent (Variables|Default|GettargetPoint))))
      (Transformation|SetActorRotation "0.000000,295.000000,0.000000")
      (Utilities|FlowControl|Delay (Variables|Default|GetfadeDelay))
      (Components|Activation|Activate (Variables|/Script/Engine.Character|GetCharacterMovement (Game|GetPlayerCharacter 0)) false)
      (bind _returnvalue (Actor|GetActorOfClass "/Game/Characters/PlayerCharacter/BP_Player.BP_Player_C"))
      (Rendering|SetVisibility (Variables|/Game/Characters/PlayerCharacter/BP_Player.BP_Player_C|GetNS_Jump _returnvalue) true false)
      (Variables|Default|SetstateIndex 3)
      (Variables|Default|SetdialogueStart false)
      ;[1 1 1] Tutorial Pop Up
      (bind _returnvalue_2 (UserInterface|CreateWidget "/Game/Assets/PlaceHolderAssets/WB_Tutorial.WB_Tutorial_C"))
      (UserInterface|Viewport|AddtoViewport _returnvalue_2 0)
      (Default|RollTutorialAnimation _returnvalue_2))))

(fn ConstructionScript
  (|CallParentFunction))