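; Self-dialogue NPC actor whose dialogue speaker is set to the player's name in its construction script.
; Entering its collision calls PlayerAdjustments after a short delay, and leaving it destroys the actor.
; After a states update it creates the tutorial widget, plays its move-tutorial animation and destroys itself, so it acts as a one-off trigger.
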(event EventPostStatesUpdate
  ;[1 1 1] Tutorial + Destroy
  (bind _returnvalue (UserInterface|CreateWidget "/Game/Assets/PlaceHolderAssets/WB_Tutorial.WB_Tutorial_C"))
  (UserInterface|Viewport|AddtoViewport _returnvalue 0)
  (Default|MoveTutorialAnimation _returnvalue)
  (Actor|DestroyActor))

(event EventEnterCollision
  ;[1 1 1] Collision Events
  (Utilities|FlowControl|Delay 0.2)
  (CallFunction|PlayerAdjustments))

(event EventExitCollision
  ;[1 1 1] Collision Events
  (Actor|DestroyActor))

(fn ConstructionScript
  (|CallParentFunction)
  (Variables|Default|SetcurrentSpeaker (Variables|Default|GetplayerName)))