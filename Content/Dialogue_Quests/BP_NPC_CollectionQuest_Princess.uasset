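; Princess NPC for a collection quest, a child Blueprint that selects its dialogue through a CurrentState index into DialogueStates.
; PostStatesUpdate moves past first-encounter dialogue, advancing state differently depending on whether the quest is accepted.
; QuestUpdate increments TotalCollected, sets its completion state and pushes the Guards trigger-quest NPC to new dialogue.
; The TotalNeeded comparison is unwired, so any single update advances both NPCs.
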(event EventQuestUpdate
  ;[1 1 1] Quest Update
  (bind _result (Math|Integer|IncrementInt (Variables|Default|GettotalCollected))
    (:%20%20
      (if true
        (Variables|Default|SetcurrentState 4)
        (bind _returnvalue (Actor|GetActorOfClass "/Game/Dialogue_Quests/BP_NPC_TriggerQuest_Guards.BP_NPC_TriggerQuest_Guards_C"))
        (Variables|/Game/Dialogue_Quests/BP_NPC.BP_NPC_C|SetcurrentState _returnvalue 2)
        (Variables|/Game/Dialogue_Quests/BP_NPC.BP_NPC_C|SetdialogueIndex _returnvalue (Utilities|Array|Get(acopy) (Variables|/Game/Dialogue_Quests/BP_NPC.BP_NPC_C|GetDialogue%20States _returnvalue) (Variables|/Game/Dialogue_Quests/BP_NPC.BP_NPC_C|GetcurrentState _returnvalue))))
      (Variables|Default|SetdialogueIndex (Utilities|Array|Get(acopy) (Variables|Default|GetDialogue%20States) (Variables|Default|GetcurrentState))))))

(event EventPostStatesUpdate
  ;[1 1 1] First Encounter Updates
  (if (Variables|Default|GetquestAccepted)
    (if (== (Variables|Default|GetcurrentState) 2)
      (Variables|Default|SetcurrentState 3))
    (elif (== (Variables|Default|GetcurrentState) 0)
      (Variables|Default|SetcurrentState 1)))
  (Variables|Default|SetdialogueIndex (Utilities|Array|Get(acopy) (Variables|Default|GetDialogue%20States) (Variables|Default|GetcurrentState))))

(fn ConstructionScript
  (|CallParentFunction))