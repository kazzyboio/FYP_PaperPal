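; BP_NPC_Princess is a quest-giving princess NPC that tracks dialogue state and a collection quest through StateIndex.
; Post-dialogue updates advance the state based on quest acceptance, while QuestUpdate counts collected items and sets the finished state.
; On completion, it fades, spawns a Static_Princess at a TargetPoint, updates BP_NPC_Guards' state and destroys itself.
; Player movement and NSJump visibility are restored after dialogue, delayed until the fade sequence when finished.
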(event Custom|Quest%20Update
  ;[1 1 1] Quest Update
  (bind _result (Math|Integer|IncrementInt (Variables|Default|GettotalCollected))
    (:%20%20
      (if (== _result (Variables|Default|GettotalNeeded))
        (Variables|Default|SetstateIndex 4)))))

(event EventReactivateMovement
  ;[1 1 1] End Dialogue
  (if (not (== (Variables|Default|GetstateIndex) 4))
    (Components|Activation|Activate (Variables|/Script/Engine.Character|GetCharacterMovement (Game|GetPlayerCharacter 0)) false)
    (bind _returnvalue (Actor|GetActorOfClass "/Game/Characters/PlayerCharacter/BP_Player.BP_Player_C"))
    (Rendering|SetVisibility (Variables|/Game/Characters/PlayerCharacter/BP_Player.BP_Player_C|GetNS_Jump _returnvalue) true false)))

(event EventPostStatesUpdate
  ;[1 1 1] First Encounter Updates
  (if (not (== (Variables|Default|GetstateIndex) 4))
    (if (Variables|Default|GetquestAccepted)
      (if (== (Variables|Default|GetstateIndex) 2)
        (Variables|Default|SetstateIndex 3))
      (elif (== (Variables|Default|GetstateIndex) 0)
        (Variables|Default|SetstateIndex 1)))
    (else
      ;[1 1 1] Quest Finish Teleport
      (CallFunction|StartFade)
      (Utilities|FlowControl|Delay (Variables|Default|GetfadeDelay))
      (Rendering|SetActorHiddenInGame true)
      (bind _returnvalue (Game|SpawnActorfromClass "/Game/Dialogue_Quests/Static_Princess.Static_Princess_C" (Variables|Default|GetSpawn%20Transform) "Undefined" 0 0))
      (Transformation|SetActorRelativeLocation _returnvalue (Transformation|GetWorldLocation (Variables|/Script/Engine.Actor|GetRootComponent (Variables|Default|GettargetPoint))))
      (bind _returnvalue_2 (Actor|GetActorOfClass "/Game/Dialogue_Quests/BP_NPC_Guards.BP_NPC_Guards_C"))
      (Variables|/Game/Dialogue_Quests/BP_NPC.BP_NPC_C|SetstateIndex _returnvalue_2 2)
      (Utilities|FlowControl|Delay (Variables|Default|GetfadeDelay))
      (Components|Activation|Activate (Variables|/Script/Engine.Character|GetCharacterMovement (Game|GetPlayerCharacter 0)) false)
      (bind _returnvalue_3 (Actor|GetActorOfClass "/Game/Characters/PlayerCharacter/BP_Player.BP_Player_C"))
      (Rendering|SetVisibility (Variables|/Game/Characters/PlayerCharacter/BP_Player.BP_Player_C|GetNS_Jump _returnvalue_3) true false)
      (Actor|DestroyActor))))

(fn ConstructionScript
  (|CallParentFunction))