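; BP_QuestItem is a quest item pickup with a configurable mesh, set from ItemMesh in the construction script.
; When BP_Player overlaps its sphere, it enables custom depth highlighting and shows a billboard prompt matching the current input device, then hides both on exit.
; PickUpItem calls the empty PickUpUpdate event, then destroys the actor.
; The glow and collect Niagara effects are deactivated on BeginPlay and never activated here.
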(event OnComponentBeginOverlap(SphereCollisionRadius)
  (params (OverlappedComponent :type Primitive%20Component%20Object%20Reference) (OtherActor :type Actor%20Object%20Reference) (OtherComp :type Primitive%20Component%20Object%20Reference) (OtherBodyIndex :type Integer) (bFromSweep :type Boolean) (SweepResult :type Hit%20Result%20Structure%20%28by%20ref%29))
  ;[1 1 1] Call Collision Events
  (Utilities|Casting|CastToBP_Player OtherActor)
  (CallFunction|EnterCollision))

(event OnComponentEndOverlap(SphereCollisionRadius)
  (params (OverlappedComponent :type Primitive%20Component%20Object%20Reference) (OtherActor :type Actor%20Object%20Reference) (OtherComp :type Primitive%20Component%20Object%20Reference) (OtherBodyIndex :type Integer))
  ;[1 1 1] Call Collision Events
  (Utilities|Casting|CastToBP_Player OtherActor)
  (CallFunction|ExitCollision))

(event Custom|Pick%20Up%20Update
  ;[1 1 1] Pick Up
)

(event Custom|Enter%20Collision
  (bind _plane (Variables|Default|GetPlane))
  ;[1 1 1] Highlight
  (Rendering|SetRenderCustomDepth (Variables|Default|GetStaticMesh) true)
  (bind _asbp_player (Utilities|Casting|CastToBP_Player (Game|GetPlayerCharacter 0)))
  (switch Utilities|FlowControl|Switch|SwitchonInputDevice (Variables|/Game/PlayerCharacter/BP_Player.BP_Player_C|GetCurrentInputDevice _asbp_player)
    (:NewEnumerator0
      (Rendering|Material|SetMaterial _plane 0 "/Game/Assets/Materials/M_Billboard_F.M_Billboard_F"))
    (:NewEnumerator1
      (Rendering|Material|SetMaterial _plane 0 "/Game/Assets/Materials/M_Billboard_B.M_Billboard_B")))
  (Rendering|SetVisibility _plane true false))

(event Custom|Exit%20Collision
  ;[1 1 1] Highlight
  (Rendering|SetRenderCustomDepth (Variables|Default|GetStaticMesh) false)
  (Rendering|SetVisibility (Variables|Default|GetPlane) false false))

(event EventPickUpItem
  ;[1 1 1] Pick Up
  (CallFunction|PickUpUpdate)
  (Actor|DestroyActor))

(event EventBeginPlay
  (Components|Activation|Deactivate (Variables|Default|GetNS_ItemGlow)))

(fn ConstructionScript
  (Components|StaticMesh|SetStaticMesh (Variables|Default|GetStaticMesh) (Variables|Default|GetitemMesh)))