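; BP_Gate is a gate actor that opens once enough pressure switches are active and closes when too few remain.
; SwitchActivated and SwitchDeactivated events adjust an active-switch count and compare it to the required count.
; The result plays or reverses the GateOpen timeline, which drives the Gate component's relative Z location, so an interrupted move reverses from its current position.
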(event Custom|SwitchDeactivated
  (Math|Integer|DecrementInt (Variables|Default|GetPressureSwitchActive)
    (:%20%20
      (if (>= (Variables|Default|GetPressureSwitchActive) (Variables|Default|GetPressureSwitchNeeded))
        (bind _gateposition (Timeline|GateOpen Play)
          (:Update
            (Transformation|SetRelativeLocation (Variables|Default|GetGate) (Math|Vector|MakeVector 0.0 0.0 _gateposition) false false)))
        (else
          (Timeline|GateOpen Reverse))))))

(event Custom|SwitchActivated
  (Math|Integer|IncrementInt (Variables|Default|GetPressureSwitchActive)
    (:%20%20
      (if (>= (Variables|Default|GetPressureSwitchActive) (Variables|Default|GetPressureSwitchNeeded))
        (bind _gateposition (Timeline|GateOpen Play)
          (:Update
            (Transformation|SetRelativeLocation (Variables|Default|GetGate) (Math|Vector|MakeVector 0.0 0.0 _gateposition) false false)))
        (else
          (Timeline|GateOpen Reverse))))))

(fn ConstructionScript)