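; BP_Hat is a hat pickup that shows its HatMaterial on a plane with a highlight and Niagara glow.
; Each player overlap applies that material to the player's hat and plays a pop sound, as the pickup stays in place.
; The first overlap also clears the highlight and glow, shows the hat-collected tutorial widget, and unlocks the existing WB_Hat_Button with a matching RowName.
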(event OnComponentBeginOverlap(re)
  (params (OverlappedComponent :type Primitive%20Component%20Object%20Reference) (OtherActor :type Actor%20Object%20Reference) (OtherComp :type Primitive%20Component%20Object%20Reference) (OtherBodyIndex :type Integer) (bFromSweep :type Boolean) (SweepResult :type Hit%20Result%20Structure%20%28by%20ref%29))
  (bind _asbp_player (Utilities|Casting|CastToBP_Player OtherActor))
  (Rendering|Material|SetMaterial (Variables|/Game/PlayerCharacter/BP_Player.BP_Player_C|GetS_Hat _asbp_player) 0 (Variables|Default|GetHatMaterial))
  (Audio|PlaySound2D "/Game/Assets/SFX/SFX_Pop_2.SFX_Pop_2" 1.0 1.0 0.0 0 0)
  (Utilities|FlowControl|DoOnce false
    (:Completed
      (Rendering|Material|SetScalarParameterValueonMaterials (Variables|Default|GetPlane) "Highlight" 0.0)
      (Components|Activation|Deactivate (Variables|Default|GetNS_ItemGlow))
      (bind _returnvalue (UserInterface|CreateWidget "/Game/Assets/UI/WB/WB_Tutorial.WB_Tutorial_C" (Game|GetPlayerController 0)))
      (UserInterface|Viewport|AddtoViewport _returnvalue 0)
      (Default|HatCollected _returnvalue)
      (bind _foundwidgets (Widget|GetAllWidgetsOfClass "/Game/Assets/UI/WB/WB_Hat_Button.WB_Hat_Button_C" false))
      (bind _array_element (Utilities|Array|ForEachLoopwithBreak _foundwidgets :!label _label)
        (:LoopBody
          (if (== (Variables|/Game/Assets/UI/WB/WB_Hat_Button.WB_Hat_Button_C|GetrowName _array_element) (Variables|Default|GetRowName))
            (Default|Unlock _array_element)
            (goto _label Break)))))))

(event EventBeginPlay
  (Rendering|Material|SetScalarParameterValueonMaterials (Variables|Default|GetPlane) "Highlight" 1.0)
  (Components|Activation|Activate (Variables|Default|GetNS_ItemGlow) false))

(fn ConstructionScript
  (Rendering|Material|SetMaterial (Variables|Default|GetPlane) 0 (Variables|Default|GetHatMaterial)))