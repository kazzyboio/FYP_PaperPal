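; BP_TableSpring is a table spring actor that launches BP_Player on overlap with its Box trigger and plays a boing sound.
; A sprinting player entering Box1 plays the hit animation sequence, destroys Cube1 and Box1, and plays a wood sound.
; After a delay of the animation's length, Box switches to OverlapAllDynamic collision so it can serve as the launch trigger.
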(event OnComponentBeginOverlap(Box)
  (params (OverlappedComponent :type Primitive%20Component%20Object%20Reference) (OtherActor :type Actor%20Object%20Reference) (OtherComp :type Primitive%20Component%20Object%20Reference) (OtherBodyIndex :type Integer) (bFromSweep :type Boolean) (SweepResult :type Hit%20Result%20Structure%20%28by%20ref%29))
  (bind _asbp_player (Utilities|Casting|CastToBP_Player OtherActor))
  (Character|LaunchCharacter _asbp_player (Variables|Default|GetLaunch%20Velocity) false false)
  (Audio|PlaySound2D "/Game/Assets/SFX/SFX_boing.SFX_boing" 1.0 1.0 0.0 0 0))

(event OnComponentBeginOverlap(Box1)
  (params (OverlappedComponent :type Primitive%20Component%20Object%20Reference) (OtherActor :type Actor%20Object%20Reference) (OtherComp :type Primitive%20Component%20Object%20Reference) (OtherBodyIndex :type Integer) (bFromSweep :type Boolean) (SweepResult :type Hit%20Result%20Structure%20%28by%20ref%29))
  (bind _asbp_player (Utilities|Casting|CastToBP_Player OtherActor))
  (if (Variables|/Game/PlayerCharacter/BP_Player.BP_Player_C|GetSprinting _asbp_player)
    (Sequencer|Player|Play (Variables|/Script/LevelSequence.LevelSequenceActor|GetSequencePlayer (Variables|Default|GetHitAnimation)) :!class /Script/MovieScene.MovieSceneSequencePlayer)
    (Components|DestroyComponent (Variables|Default|GetCube1))
    (Audio|PlaySound2D "/Game/Assets/SFX/SFX_Wood.SFX_Wood" 1.0 1.0 0.0 0 0)
    (Utilities|FlowControl|Delay (Variables|Default|GetanimationLength))
    (Collision|SetCollisionProfileName (Variables|Default|GetBox) "OverlapAllDynamic" true :!class /Script/Engine.PrimitiveComponent)))

(fn ConstructionScript)