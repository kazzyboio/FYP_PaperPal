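; BP_Plate is a pressure plate actor that signals a linked gate when player character 0 steps on or off it.
; Overlap begin and end call SwitchActivated and SwitchDeactivated on GateToActivate, ignoring all other actors.
; The same events play and reverse the PlatePosition timeline, which sets the Switch component's relative Z to animate the plate.
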(event Collision|EventActorBeginOverlap
  (params (OtherActor :type Actor%20Object%20Reference))
  (if (== OtherActor (Game|GetPlayerCharacter 0))
    (Default|SwitchActivated (Variables|Default|GetGateToActivate))
    (bind _switchposition (Timeline|PlatePosition Play)
      (:Update
        (Transformation|SetRelativeLocation (Variables|Default|GetSwitch) (Math|Vector|MakeVector 0.0 0.0 _switchposition) false false)))))

(event Collision|EventActorEndOverlap
  (params (OtherActor :type Actor%20Object%20Reference))
  (if (== OtherActor (Game|GetPlayerCharacter 0))
    (Default|SwitchDeactivated (Variables|Default|GetGateToActivate))
    (bind _switchposition (Timeline|PlatePosition Reverse)
      (:Update
        (Transformation|SetRelativeLocation (Variables|Default|GetSwitch) (Math|Vector|MakeVector 0.0 0.0 _switchposition) false false)))))

(fn ConstructionScript)