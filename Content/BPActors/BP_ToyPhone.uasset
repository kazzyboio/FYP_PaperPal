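; BP_ToyPhone is an interactable toy phone actor that plays a song when the player presses Interact nearby.
; The Box overlap with BP_Player toggles input, a custom depth highlight on the mesh, and a Plane's visibility.
; Pressing Interact plays the Song set at BeginPlay, and an IsPlaying flag with a fixed delay blocks retriggering while it plays.
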(event OnComponentBeginOverlap(Box)
  (params (OverlappedComponent :type Primitive%20Component%20Object%20Reference) (OtherActor :type Actor%20Object%20Reference) (OtherComp :type Primitive%20Component%20Object%20Reference) (OtherBodyIndex :type Integer) (bFromSweep :type Boolean) (SweepResult :type Hit%20Result%20Structure%20%28by%20ref%29))
  (Utilities|Casting|CastToBP_Player OtherActor)
  (Input|EnableInput (Game|GetPlayerController 0))
  (Rendering|SetRenderCustomDepth (Variables|Default|GetStaticMesh) true)
  (Rendering|SetVisibility (Variables|Default|GetPlane) true false))

(event OnComponentEndOverlap(Box)
  (params (OverlappedComponent :type Primitive%20Component%20Object%20Reference) (OtherActor :type Actor%20Object%20Reference) (OtherComp :type Primitive%20Component%20Object%20Reference) (OtherBodyIndex :type Integer))
  (Utilities|Casting|CastToBP_Player OtherActor)
  (Input|DisableInput (Game|GetPlayerController 0))
  (Rendering|SetRenderCustomDepth (Variables|Default|GetStaticMesh) false)
  (Rendering|SetVisibility (Variables|Default|GetPlane) false false))

(event EventBeginPlay
  (Audio|Components|Audio|SetSound (Variables|Default|GetAudio) (Variables|Default|GetSong)))

(event Input|ActionEvents|InputActionInteract
  (params (Key :type Key%20Structure :default "None"))
  (:Pressed
    (if (not (Variables|Default|GetIsPlaying?))
      (Variables|Default|SetIsPlaying? true)
      (Audio|Components|Audio|Play (Variables|Default|GetAudio) 0.0)
      (Utilities|FlowControl|Delay 15.0)
      (Variables|Default|SetIsPlaying? false))))

(fn ConstructionScript)