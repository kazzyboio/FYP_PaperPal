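; BP_OutdoorAmbience is an actor that plays outdoor ambient audio with occasional extra sounds.
; On BeginPlay it assigns sounds to three audio components and starts the outdoor one.
; A looping timer, whose interval of a few minutes is randomized once at start, fires RandomSound, which plays either the ONP or the Walls ambience at random.
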(event Custom|RandomSound
  (switch int (Math|Random|RandomIntegerinRange 0 1)
    (:0
      (Audio|Components|Audio|Play (Variables|Default|GetONPAudio) 0.0))
    (:1
      (Audio|Components|Audio|Play (Variables|Default|GetWallsAudio) 0.0))))

(event EventBeginPlay
  (Audio|Components|Audio|SetSound (Variables|Default|GetOutdoorAudio) (Variables|Default|GetOutdoorAmbience))
  (Audio|Components|Audio|SetSound (Variables|Default|GetWallsAudio) (Variables|Default|GetWalls%20Ambience))
  (Audio|Components|Audio|SetSound (Variables|Default|GetONPAudio) (Variables|Default|GetONP%20Ambience))
  (Audio|Components|Audio|Play (Variables|Default|GetOutdoorAudio) 0.0)
  (Utilities|Time|SetTimerbyEvent (delegate Custom|RandomSound) (Math|Random|RandomFloatinRange 1.2e+02 3e+02) true))

(fn ConstructionScript)