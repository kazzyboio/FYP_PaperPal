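; BP_Water is a water hazard actor that sends the player back to a spawn point when they fall in.
; On overlap it disables input, fires the player's NSFormSwitch effect, waits a second, then moves the player to SpawnPoint, restores input and unhides the mesh and hat.
; If the player is stinky, a one-time branch tints the water material brown and clears that state.
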(event OnComponentHit(water)
  (params (HitComponent :type Primitive%20Component%20Object%20Reference) (OtherActor :type Actor%20Object%20Reference) (OtherComp :type Primitive%20Component%20Object%20Reference) (NormalImpulse :type Vector :default "0, 0, 0") (Hit :type Hit%20Result%20Structure%20%28by%20ref%29)))

(event OnComponentBeginOverlap(water)
  (params (OverlappedComponent :type Primitive%20Component%20Object%20Reference) (OtherActor :type Actor%20Object%20Reference) (OtherComp :type Primitive%20Component%20Object%20Reference) (OtherBodyIndex :type Integer) (bFromSweep :type Boolean) (SweepResult :type Hit%20Result%20Structure%20%28by%20ref%29))
  (bind _asbp_player (Utilities|Casting|CastToBP_Player OtherActor))
  (Input|DisableInput _asbp_player (Game|GetPlayerController 0))
  (Components|Activation|Activate (Variables|/Game/PlayerCharacter/BP_Player.BP_Player_C|GetNS_FormSwitch _asbp_player) true)
  (Utilities|FlowControl|Delay 1.0)
  (Transformation|SetRelativeLocation (Variables|/Script/Engine.Actor|GetRootComponent _asbp_player) (Variables|Default|GetSpawn%20Point) false false)
  (Input|EnableInput _asbp_player (Game|GetPlayerController 0))
  (Development|SetHiddeninGame (Variables|/Script/Engine.Character|GetMesh _asbp_player) false false)
  (bind _returnvalue (Actor|GetActorOfClass "/Game/PlayerCharacter/BP_Player.BP_Player_C"))
  ;[1 1 1] Turn water brown when stinky
  (if (Variables|/Game/PlayerCharacter/BP_Player.BP_Player_C|GetisStinky _returnvalue)
    (Utilities|FlowControl|DoOnce false
      (:Completed
        (Rendering|Material|SetVectorParameterValueonMaterials (Variables|Default|Getwater) "Colour" "0.322917,0.099803,0.031669")
        (Variables|/Game/PlayerCharacter/BP_Player.BP_Player_C|SetisStinky _returnvalue false)))))

(event EventBeginPlay)

(event Collision|EventActorBeginOverlap
  (params (OtherActor :type Actor%20Object%20Reference)))

(event EventTick
  (params (DeltaSeconds :type Float%20%28single-precision%29)))

(fn ConstructionScript)

(fn NewFunction0)