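; BP_Plate_Castle is a pressure plate that drives a linked castle gate when the player character steps on or off it.
; Overlap begin and end call activate and deactivate on GateToActivate and play or reverse a timeline that moves the switch's Z position.
; Each timeline update also looks up BP_NPC_MrTomatoHead and calls GateOpened on it while PastGate is false, including during reverse playback.
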(event Collision|EventActorBeginOverlap
  (params (OtherActor :type Actor%20Object%20Reference))
  (if (== OtherActor (Game|GetPlayerCharacter 0))
    (Default|SwitchActivated (Variables|Default|GetGateToActivate))
    (bind _switchposition (Timeline|Timeline_0 Play)
      (:Update
        (Transformation|SetRelativeLocation (Variables|Default|GetSwitch) (Math|Vector|MakeVector 0.0 0.0 _switchposition) false false)
        (bind _returnvalue (Actor|GetActorOfClass "/Game/Dialogue_Quests/NPC/BP_NPC_MrTomatoHead.BP_NPC_MrTomatoHead_C"))
        (if (not (Variables|/Game/Dialogue_Quests/NPC/BP_NPC_MrTomatoHead.BP_NPC_MrTomatoHead_C|GetpastGate _returnvalue))
          (Default|GateOpened _returnvalue))))))

(event Collision|EventActorEndOverlap
  (params (OtherActor :type Actor%20Object%20Reference))
  (if (== OtherActor (Game|GetPlayerCharacter 0))
    (Default|SwitchDeactivated (Variables|Default|GetGateToActivate))
    (bind _switchposition (Timeline|Timeline_0 Reverse)
      (:Update
        (Transformation|SetRelativeLocation (Variables|Default|GetSwitch) (Math|Vector|MakeVector 0.0 0.0 _switchposition) false false)
        (bind _returnvalue (Actor|GetActorOfClass "/Game/Dialogue_Quests/NPC/BP_NPC_MrTomatoHead.BP_NPC_MrTomatoHead_C"))
        (if (not (Variables|/Game/Dialogue_Quests/NPC/BP_NPC_MrTomatoHead.BP_NPC_MrTomatoHead_C|GetpastGate _returnvalue))
          (Default|GateOpened _returnvalue))))))

(fn ConstructionScript
  (|CallParentFunction))