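; BP_BigBlock is a block the player knocks down by sprinting into it, as part of Joshzilla's quest.
; Once that NPC's quest is accepted, the block highlights until knocked.
; Sprinting overlaps shake the camera and count hits; at the needed total it plays a cutscene, triggers the NPC's auto dialogue, shakes again and disables its trigger.
; A Spawn event reveals the block, enables overlaps and blocking collision, and destroys the BigBlockPile actor.
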(event OnComponentBeginOverlap(Box)
  (params (OverlappedComponent :type Primitive%20Component%20Object%20Reference) (OtherActor :type Actor%20Object%20Reference) (OtherComp :type Primitive%20Component%20Object%20Reference) (OtherBodyIndex :type Integer) (bFromSweep :type Boolean) (SweepResult :type Hit%20Result%20Structure%20%28by%20ref%29))
  ;[1 1 1] Knock Down
  (bind _asbp_player (Utilities|Casting|CastToBP_Player OtherActor))
  (if (Variables|/Game/PlayerCharacter/BP_Player.BP_Player_C|GetSprinting _asbp_player)
    (Camera|PlayWorldCameraShake "/Game/BPActors/BP_CameraShake.BP_CameraShake_C" (Transformation|GetActorLocation (Game|GetPlayerCameraManager 0)) 5e+02 5e+02)
    (bind _result (Math|Integer|IncrementInt (Variables|Default|GetTotalHit))
      (:%20%20
        (if (== _result (Variables|Default|GetTotalNeeded))
          (Utilities|FlowControl|DoOnce false
            (:Completed
              (Sequencer|Player|Play (Variables|/Script/LevelSequence.LevelSequenceActor|GetSequencePlayer (Variables|Default|GetCutscene)) :!class /Script/MovieScene.MovieSceneSequencePlayer)
              (Variables|Default|SetKnocked true)
              (Rendering|Material|SetScalarParameterValueonMaterials (Variables|Default|GetCube1) "Highlight" 0.0)
              (bind _returnvalue (Actor|GetActorOfClass "/Game/Dialogue_Quests/NPC/BP_NPC_Joshzilla.BP_NPC_Joshzilla_C"))
              (Default|AutoDialogue _returnvalue)
              (Utilities|FlowControl|Delay 1.9)
              (Camera|PlayWorldCameraShake "/Game/BPActors/BP_CameraShake_2.BP_CameraShake_2_C" (Transformation|GetActorLocation (Game|GetPlayerCameraManager 0)) 5e+02 5e+02)
              (Collision|SetCollisionEnabled (Variables|Default|GetBox) "NoCollision"))))))))

(event Custom|Spawn
  ;[1 1 1] Spawn In
  (Rendering|SetActorHiddenInGame false)
  (Variables|/Script/Engine.PrimitiveComponent|SetbGenerateOverlapEvents (Variables|Default|GetBox) true)
  (Collision|SetCollisionProfileName (Variables|Default|GetCube) "BlockAllDynamic" true :!class /Script/Engine.PrimitiveComponent)
  (Actor|DestroyActor (Variables|Default|GetbigBlockPile)))

(event EventTick
  (params (DeltaSeconds :type Float%20%28single-precision%29))
  (if (not (Variables|Default|Getknocked))
    (bind _returnvalue (Actor|GetActorOfClass "/Game/Dialogue_Quests/NPC/BP_NPC_Joshzilla.BP_NPC_Joshzilla_C"))
    (if (Variables|/Game/Dialogue_Quests/NPC/BP_NPC_Joshzilla.BP_NPC_Joshzilla_C|GetquestAccepted _returnvalue)
      (Utilities|FlowControl|DoOnce false
        (:Completed
          (Rendering|Material|SetScalarParameterValueonMaterials (Variables|Default|GetCube1) "Highlight" 1.0))))))

(fn ConstructionScript)