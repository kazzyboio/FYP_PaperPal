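; BP_Radio is an interactable radio actor that the player toggles on and off with the F key.
; Entering its box trigger as BP_Player enables input, outlines the mesh via custom depth and shows a plane; leaving reverses this.
; Each toggle plays a click sound; switching on starts the song after a short delay with a music-note Niagara effect, and switching off stops both.
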(event OnComponentBeginOverlap(Box)
  (params (OverlappedComponent :type Primitive%20Component%20Object%20Reference) (OtherActor :type Actor%20Object%20Reference) (OtherComp :type Primitive%20Component%20Object%20Reference) (OtherBodyIndex :type Integer) (bFromSweep :type Boolean) (SweepResult :type Hit%20Result%20Structure%20%28by%20ref%29))
  ;[1 1 1] Input/Highlight
  (Utilities|Casting|CastToBP_Player OtherActor)
  (Input|EnableInput (Game|GetPlayerController 0))
  (Rendering|SetRenderCustomDepth (Variables|Default|GetStaticMesh) true)
  (Rendering|SetVisibility (Variables|Default|GetPlane) true false))

(event OnComponentEndOverlap(Box)
  (params (OverlappedComponent :type Primitive%20Component%20Object%20Reference) (OtherActor :type Actor%20Object%20Reference) (OtherComp :type Primitive%20Component%20Object%20Reference) (OtherBodyIndex :type Integer))
  ;[1 1 1] Input/Highlight
  (Utilities|Casting|CastToBP_Player OtherActor)
  (Input|DisableInput (Game|GetPlayerController 0))
  (Rendering|SetRenderCustomDepth (Variables|Default|GetStaticMesh) false)
  (Rendering|SetVisibility (Variables|Default|GetPlane) false false))

(event EventBeginPlay
  (Audio|Components|Audio|SetSound (Variables|Default|GetStartEndAudio) (Variables|Default|GetRadio%20Click))
  (Audio|Components|Audio|SetSound (Variables|Default|GetAudio1) (Variables|Default|GetRadioSong1))
  (Components|Activation|Deactivate (Variables|Default|GetNS_MusicNotes)))

(event Input|KeyboardEvents|F
  (params (Key :type Key%20Structure :default "None"))
  (bind _ns_musicnotes (Variables|Default|GetNS_MusicNotes))
  (bind _audio1 (Variables|Default|GetAudio1))
  (:Pressed
    (if (Variables|Default|GetIsPlaying?)
      (Audio|Components|Audio|Play (Variables|Default|GetStartEndAudio) 0.0)
      (Audio|Components|Audio|Stop _audio1)
      (Variables|Default|SetIsPlaying? false)
      (Components|Activation|Deactivate _ns_musicnotes)
      (else
        (Audio|Components|Audio|Play (Variables|Default|GetStartEndAudio) 0.0)
        (Utilities|FlowControl|Delay 0.7)
        (Audio|Components|Audio|Play _audio1 0.0)
        (Variables|Default|SetIsPlaying? true)
        (Components|Activation|Activate _ns_musicnotes false)))))

(fn ConstructionScript)